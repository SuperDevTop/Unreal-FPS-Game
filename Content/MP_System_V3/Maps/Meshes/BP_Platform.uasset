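; BP_Platform is an elevator that carries BP_MPS_Master actors between its placed position and a fixed height above it, both computed in the construction script.
; Overlapping Box raises it via the Movement timeline, or lowers it after a short delay if already at the top.
; Leaving Box stops the rise, and overlapping IsOnTop while not moving triggers descent.
; Both timelines feed VInterpTo as DeltaTime to set Box's location.
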(event `self.Box.OnComponentBeginOverlap`
  (params (OverlappedComponent :type "PrimitiveComponent Object Reference") (OtherActor :type "Actor Object Reference") (OtherComp :type "PrimitiveComponent Object Reference") (OtherBodyIndex :type Integer) (bFromSweep :type Boolean) (SweepResult :type "HitResult Structure (by ref)"))
  (bind _box (`self.Box`))
  (bind _box_2 (`self.Box`))
  (bind _targetlocation (`self.TargetLocation`))
  (cast `/Game/MP_System_V3/Game/Blueprints/Core/BP_MPS_Master` OtherActor)
  (if (`self.IsOnTopPlatform?`)
    (`KismetSystemLibrary.Delay` 0.5)
    (bind (_direction _interp) (`Timeline|ReverseMovement` :!via `PlayFromStart` :!label _label)
      (:`Update`
        (`SceneComponent.K2_SetWorldLocation` _box (`KismetMathLibrary.VInterpTo` (`SceneComponent.K2_GetComponentLocation` _box) (`self.InitialLocation`) _interp 0.1) false false)
        (set `self.IsOnTopPlatform?` false)))
    (else
      (`/Engine/EditorBlueprintResources/StandardMacros.DoOnce` false :!label _label_2
        (:`Completed`
          (set `self.IsMoving?` true)
          (bind (_direction_2 _interp_2) (`Timeline|Movement` :!via `PlayFromStart` :!label _label_3)
            (:`Update`
              (`SceneComponent.K2_SetWorldLocation` _box_2 (`KismetMathLibrary.VInterpTo` (`self.InitialLocation`) _targetlocation _interp_2 2.0) false false)
              (if (== (`SceneComponent.K2_GetComponentLocation` _box_2) _targetlocation)
                (set `self.IsOnTopPlatform?` true)))))))))

(event `self.Box.OnComponentEndOverlap`
  (params (OverlappedComponent :type "PrimitiveComponent Object Reference") (OtherActor :type "Actor Object Reference") (OtherComp :type "PrimitiveComponent Object Reference") (OtherBodyIndex :type Integer))
  (cast `/Game/MP_System_V3/Game/Blueprints/Core/BP_MPS_Master` OtherActor)
  (`|ExecutionSequence`
    (:`then_0`
      (goto _label_2 :!via `Reset`))
    (:`then_1`
      (set `self.IsMoving?` false)
      (goto _label_3 :!via `Stop`))))

(event `self.IsOnTop?.OnComponentBeginOverlap`
  (params (OverlappedComponent :type "PrimitiveComponent Object Reference") (OtherActor :type "Actor Object Reference") (OtherComp :type "PrimitiveComponent Object Reference") (OtherBodyIndex :type Integer) (bFromSweep :type Boolean) (SweepResult :type "HitResult Structure (by ref)"))
  (cast `/Game/MP_System_V3/Game/Blueprints/Core/BP_MPS_Master` OtherActor)
  (if (not (`self.IsMoving?`))
    (set `self.IsOnTopPlatform?` false)
    (goto _label :!via `PlayFromStart`)))

(fn `UserConstructionScript`
  (bind (_returnvalue_x _returnvalue_y _returnvalue_z) (`KismetMathLibrary.BreakVector` (`SceneComponent.K2_GetComponentLocation` (`self.Box`))))
  (bind _output_get (set `self.InitialLocation` (`KismetMathLibrary.MakeVector` _returnvalue_x _returnvalue_y _returnvalue_z)))
  (set `self.TargetLocation` (`KismetMathLibrary.MakeVector` (.x _output_get) (.y _output_get) (+ (.z _output_get) 750.0))))