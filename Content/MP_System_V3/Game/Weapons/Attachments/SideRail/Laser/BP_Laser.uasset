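; Laser sight weapon attachment that draws a beam and a light dot where it points.
; BeginPlay snaps the mesh to the "Laser" socket after a short delay and caches the owning MPS character's camera.
; Each post-update tick traces from the camera, setting the beam end and moving a distance-scaled point light to the hit.
; SwitchTraceEnd changes the trace direction between weapon and camera based on blocked, aiming, third-person and montage state.
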(event `self.ReceiveBeginPlay`
  ;[0.3005 0.3005 0.3005] Connect
  (`ActorComponent.SetTickGroup` (`self.Mesh`) "TG_PostUpdateWork")
  (`KismetSystemLibrary.Delay` 0.2)
  (bind _start (`self.Start`)
    (:`then`
      (`SceneComponent.K2_SetWorldLocation` (`self.Mesh`) (`SceneComponent.GetSocketLocation` _start "Laser") false false)
      (bind _output_get (set `self.MPS` (cast `/Game/MP_System_V3/Game/Blueprints/Core/BP_MPS_Master` (`self.GetInstigator`) :!pure true)))
      (set `self.Camera` (`/Game/MP_System_V3/Game/Blueprints/Core/BP_MPS_Master.Camera` _output_get)))
    (:`else`)))

(event `self.ReceiveTick`
  (params (DeltaSeconds :type "Float (single-precision)"))
  (bind _returnvalue (`self.SwitchTraceEnd`))
  (bind _pointlight (`self.PointLight`))
  (bind _start (`self.Start`))
  ;[0.3 0.3 0.3] Laser Target Acquisition
  (`/Engine/EditorBlueprintResources/StandardMacros.IsValid` (`self.Start`)
    (:`Is Valid`
      (`/Engine/EditorBlueprintResources/StandardMacros.IsValid` (`self.Camera`)
        (:`Is Valid`
          (bind _outhit (`KismetSystemLibrary.LineTraceSingle` (`SceneComponent.K2_GetComponentLocation` (`self.Camera`)) (+ (`SceneComponent.GetSocketLocation` (select `bool` _returnvalue :`false` _start :`true` (`self.Camera`) :!type "SceneComponent Object Reference") "Laser") (* (`KismetMathLibrary.SelectVector` (`SceneComponent.GetRightVector` _start) (`SceneComponent.GetForwardVector` (`self.Camera`)) _returnvalue) 10000.0)) "TraceTypeQuery1" false (`|MakeArray` (`self.GetOwner`)) "None" true (struct :`R` 0.012519 :`B` 1.0 :`A` 1.0)))
          (bind (_bblockinghit _binitialoverlap _time _distance _location _impactpoint _normal _impactnormal _physmat _hitactor _hitcomponent _hitbonename _bonename _hititem _elementindex _faceindex _tracestart _traceend) (`GameplayStatics.BreakHitResult` _outhit))
          (`ParticleSystemComponent.SetBeamEndPoint` (`self.Laser`) 0 (`KismetMathLibrary.SelectVector` _impactpoint _traceend _bblockinghit))
          (`SceneComponent.K2_SetWorldLocation` _pointlight _location false false)
          (`LocalLightComponent.SetAttenuationRadius` _pointlight (`KismetMathLibrary.FClamp` (/ _distance 400.0) 1.0 5.0)))))))

(fn `SwitchTraceEnd`
  (returns (ReturnValue :type Boolean))
  (bind _mps (`self.MPS`))
  (return (or (`/Game/MP_System_V3/Game/Blueprints/Core/BP_MPS_Master.IsBlocked?` _mps) (not (`/Game/MP_System_V3/Game/Blueprints/Core/BP_MPS_Master.IsAiming?` _mps)) (not (`/Game/MP_System_V3/Game/Blueprints/Core/BP_MPS_Master.IsTPC?` _mps)) (!= (`Character.GetCurrentMontage` _mps) null))))

(fn `UserConstructionScript`)