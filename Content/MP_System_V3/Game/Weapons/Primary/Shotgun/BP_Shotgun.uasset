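; BP_Shotgun is a shotgun primary weapon that extends a parent weapon class.
; On BeginPlay it runs the parent logic and then toggles its aim pose.
; After the parent construction script, it reads the two characters before the last two of WeaponID.
; If that segment is "00", it sets a fixed underbarrel enum value and passes its name to MCUnderbarrelAttachment.
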(event `self.ReceiveBeginPlay`
  (`parent.ReceiveBeginPlay`)
  (`self.ToggleAimPose`))

(fn `UserConstructionScript`
  (`parent.UserConstructionScript`)
  (if (`KismetStringLibrary.EqualEqual_StrStr` (`KismetStringLibrary.Right` (`KismetStringLibrary.LeftChop` (`self.WeaponID`) 2) 2) "00")
    (bind _output_get (set `self.Underbarrel_ID` "NewEnumerator11"))
    (`self.MC_UnderbarrelAttachment` (`KismetStringLibrary.Conv_StringToName` (`|GetEnumeratorNameAsString` _output_get)))))