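; Multiplayer player character Blueprint that applies mesh, vest and material choices from the player controller and adds hotkey camera tools.
; The construction script slaves the vest to the body mesh's pose.
; Keys toggle a helmet cine camera and a runtime-created weapon camera socketed to the active weapon, flip the latter, and hide widgets.
; The SlideCam macro uses a Gate and Delay loop to nudge the weapon camera while offset keys are held.
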(event `self.ReceiveBeginPlay`
  (bind _playercontroller (`/Game/MP_System_V3/Game/Blueprints/Core/FL_MPS.PlayerController_MPS`))
  ;[0.3005 0.3005 0.3005] Setup Player Data
  (`SkinnedMeshComponent.SetSkinnedAssetAndUpdate` (`self.Mesh`) (`/Game/MP_System_V3/Game/Blueprints/Core/PC_MPS.Player_MainMesh` _playercontroller) true)
  (`SkinnedMeshComponent.SetSkinnedAssetAndUpdate` (`self.Vest`) (`/Game/MP_System_V3/Game/Blueprints/Core/PC_MPS.Player_SecondaryMesh` _playercontroller) true)
  (`PrimitiveComponent.SetMaterial` (`self.Mesh`) 0 (`/Game/MP_System_V3/Game/Blueprints/Core/PC_MPS.Player_MainMaterial` _playercontroller)))

(event `Key|N`
  (params (Key :type "Key Structure"))
  ;[0.3005 0.3005 0.3005] Toggel Helmet Cam
  (:`Pressed`
    (`/Engine/EditorBlueprintResources/StandardMacros.FlipFlop`
      (:`A`
        (`ActorComponent.SetActive` (`self.CineCamera`) true false)
        (`ActorComponent.SetActive` (`self.Camera`) false false))
      (:`B`
        (`ActorComponent.SetActive` (`self.CineCamera`) false false)
        (`ActorComponent.SetActive` (`self.Camera`) true false)))))

(event `Key|M`
  (params (Key :type "Key Structure"))
  (bind _cineweapon (`self.CineWeapon`))
  ;[0.3005 0.3005 0.3005] Toggle Weapon Cam & Set Location
  (:`Pressed`
    (`self.CineWeapon`
      (:`then`
        _)
      (:`else`
        (bind _returnvalue (`AddComponent|NODE_AddCineCameraComponent-0`))
        (set `self.CineWeapon` _returnvalue)))
    (`/Engine/EditorBlueprintResources/StandardMacros.FlipFlop`
      (:`A`
        (`ActorComponent.SetActive` (`self.CineWeapon`) true false)
        (`ActorComponent.SetActive` (`self.Camera`) false false)
        (`ActorComponent.SetActive` (`self.CineCamera`) false false)
        (`SceneComponent.K2_AttachToComponent` (`self.CineWeapon`) (`/Game/MP_System_V3/Game/Blueprints/Core/BP_InteractionMaster.Item` (`self.ActiveWeapon`)) (select `int` (`self.ActiveSlot`) :`0` "Barrel" :`1` "charging_handle" :!type "Name") "SnapToTarget" "SnapToTarget" "KeepRelative" true)
        (`SceneComponent.K2_SetRelativeRotation` _cineweapon (struct :`Yaw` -90.0) false false)
        (`SceneComponent.K2_SetRelativeLocation` _cineweapon (select `int` (`self.ActiveSlot`) :`0` (-7.5 5.0 10.0) :`1` (-7.5 5.0 5.0) :!type "Vector Structure") false false))
      (:`B`
        (`ActorComponent.SetActive` (`self.CineWeapon`) false false)
        (`ActorComponent.SetActive` (`self.Camera`) true false)
        (`ActorComponent.SetActive` (`self.CineCamera`) true false)))))

(event `Key|Six`
  (params (Key :type "Key Structure"))
  ;[0.3005 0.3005 0.3005] Weapon Cam X Offset
  (:`Pressed`
    (`self.SlideCam` 1.0 :!label _label))
  (:`Released`
    (goto _label :!via `Close`)))

(event `Key|Eight`
  (params (Key :type "Key Structure"))
  ;[0.3005 0.3005 0.3005] Weapon Cam Y Offset
  (:`Pressed`
    (`self.SlideCam` 0.0 1.0 :!label _label_2))
  (:`Released`
    (goto _label_2 :!via `Close`)))

(event `Key|Hyphen`
  (params (Key :type "Key Structure"))
  ;[0.3005 0.3005 0.3005] Weapon Cam Z Offset
  (:`Pressed`
    (`self.SlideCam` 0.0 0.0 1.0 :!label _label_3))
  (:`Released`
    (goto _label_3 :!via `Close`)))

(event `Key|Period`
  (params (Key :type "Key Structure"))
  ;[0.3005 0.3005 0.3005] Hide Widgets
  (:`Pressed`
    (bind _foundwidgets (`WidgetBlueprintLibrary.GetAllWidgetsOfClass` "/Script/UMG.UserWidget"))
    (for _array_element _foundwidgets
      (`Widget.SetVisibility` _array_element "Hidden"))))

(event `Key|Seven`
  (params (Key :type "Key Structure"))
  ;[0.3005 0.3005 0.3005] Weapon Cam X Offset
  (:`Pressed`
    (`self.SlideCam` -1.0 :!label _label_4))
  (:`Released`
    (goto _label_4 :!via `Close`)))

(event `Key|Nine`
  (params (Key :type "Key Structure"))
  ;[0.3005 0.3005 0.3005] Weapon Cam Y Offset
  (:`Pressed`
    (`self.SlideCam` 0.0 -1.0 :!label _label_5))
  (:`Released`
    (goto _label_5 :!via `Close`)))

(event `Key|Equals`
  (params (Key :type "Key Structure"))
  ;[0.3005 0.3005 0.3005] Weapon Cam Z Offset
  (:`Pressed`
    (`self.SlideCam` 0.0 0.0 -1.0 :!label _label_6))
  (:`Released`
    (goto _label_6 :!via `Close`)))

(event `Key|Comma`
  (params (Key :type "Key Structure"))
  ;[0.3005 0.3005 0.3005] Weapon Cam 180° Rotation
  (:`Pressed`
    (`/Engine/EditorBlueprintResources/StandardMacros.FlipFlop`
      (:`A`
        (`SceneComponent.K2_SetRelativeRotation` (`self.CineWeapon`) (struct :`Yaw` 90.0) false false))
      (:`B`
        (`SceneComponent.K2_SetRelativeRotation` (`self.CineWeapon`) (struct :`Yaw` -90.0) false false)))))

(fn `UserConstructionScript`
  (`parent.UserConstructionScript`)
  (`SkinnedMeshComponent.SetLeaderPoseComponent` (`self.Vest`) (`self.Mesh`) false))