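; BP_Ragdoll is an animated skeletal mesh actor that moves in a repeating loop and collapses into a ragdoll when damaged.
; A timeline offsets the mesh by Movement each update, snapping it back to its construction-time transform when finished.
; Damage stops the timeline and enables physics.
; After a retriggerable delay, a freshly created component replaces the ragdolled mesh at the start transform, restoring animation, Ragdoll collision profile and movement.
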(event `self.ReceiveAnyDamage`
  (params (Damage :type "Float (single-precision)") (DamageType :type "DamageType Object Reference") (InstigatedBy :type "Controller Object Reference") (DamageCauser :type "Actor Object Reference"))
  (bind _skeletalmesh (`self.SkeletalMesh`))
  (`|ExecutionSequence`
    (:`then_0`
      (`PrimitiveComponent.SetSimulatePhysics` (`self.SkeletalMesh`) true)
      (`SkeletalMeshComponent.Stop` (`self.SkeletalMesh`))
      (`KismetSystemLibrary.RetriggerableDelay` 3.0)
      (bind _returnvalue (`AddComponent|NODE_AddSkeletalMeshComponent-0`))
      (`SkinnedMeshComponent.SetSkinnedAssetAndUpdate` _returnvalue (`SkinnedMeshComponent.SkeletalMesh` (`self.SkeletalMesh`)) true)
      (`SceneComponent.K2_SetWorldTransform` _returnvalue (`self.Transform`) false false)
      (`ActorComponent.K2_DestroyComponent` (`self.SkeletalMesh`))
      (bind _output_get (set `self.SkeletalMesh` _returnvalue))
      (`SkeletalMeshComponent.OverrideAnimationData` (`self.SkeletalMesh`) (`self.Animation`) true true 0.0 1.0)
      (`PrimitiveComponent.SetCollisionProfileName` _output_get "Ragdoll" true)
      (`Timeline|01` :!via `PlayFromStart` :!label _label
        (:`Update`
          (`SceneComponent.K2_SetWorldLocation` _skeletalmesh (+ (`SceneComponent.K2_GetComponentLocation` _skeletalmesh) (`self.Movement`)) false true))
        (:`Finished`
          (`SceneComponent.K2_SetWorldTransform` (`self.SkeletalMesh`) (`self.Transform`) false true)
          (goto _label :!via `PlayFromStart`))))
    (:`then_1`
      (goto _label :!via `Stop`))))

(event `self.ReceiveBeginPlay`
  (goto _label :!via `PlayFromStart`))

(fn `UserConstructionScript`
  (set `self.Transform` (`SceneComponent.K2_GetComponentToWorld` (`self.SkeletalMesh`)))
  (`SkeletalMeshComponent.OverrideAnimationData` (`self.SkeletalMesh`) (`self.Animation`) true true 0.0 1.0))