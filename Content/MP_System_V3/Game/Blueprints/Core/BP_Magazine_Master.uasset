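; BP_Magazine_Master is the base ammo magazine item pickup, named after the weapon it supplies.
; Its construction script sets the item type, display name and mesh, and reads the DT_Weapons row for that weapon to get clamped ammo, slot and weapon type.
; It returns itself through the I_Magazine interface function.
; On destruction it calls a client event that plays a 2D pickup sound.
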(event `self.ReceiveDestroyed`
  (`self.Client_PlayPickupSound`))

(event `Client_PlayPickupSound`
  (`GameplayStatics.PlaySound2D` "/Game/MP_System_V3/Game/Sounds/Cue/AmmoPickup_Cue.AmmoPickup_Cue" 1.0 1.0 0.0 null null))

(fn `DataTable`
  (bind _returnvalue (`|GetDataTableRow` "/Game/MP_System_V3/Game/Blueprints/DataTables/DT_Weapons.DT_Weapons" (`self.Name`))
    (:`then`
      (set `self.DT_AmmoMag` (`KismetMathLibrary.Clamp` (`self.Ammo`) 0 (`.AmmoMag_19_752EA06E412F98C36FF42C9E397F3B96` (break `/Game/MP_System_V3/Game/Blueprints/Structs/ST_WeaponCore` (break `/Game/MP_System_V3/Game/Blueprints/Structs/ST_WeaponData` _returnvalue)))))
      (bind ((`InventorySlot_22_8AE0E62544EF72051D2D64A9D357ECD9` _inventoryslot) (`WeaponType_25_374001744D365AD0A56B368FE648734B` _weapontype)) (break `/Game/MP_System_V3/Game/Blueprints/Structs/ST_Weapon_Params` (`.Parameters_7_B4C44D104F192554522E0AA5E66526D4` (break `/Game/MP_System_V3/Game/Blueprints/Structs/ST_WeaponData` _returnvalue))))
      (set `self.DT_Slot` (`KismetMathLibrary.Conv_ByteToInt` _inventoryslot))
      (set `self.DT_Type` _weapontype))))

(fn `I_Magazine`
  (returns (Magazine :type "/Game/MP_System_V3/Game/Blueprints/Core/BP_Magazine_Master Object Reference"))
  (return self))

(fn `UserConstructionScript`
  (`parent.UserConstructionScript`)
  (set `self.ItemType` "NewEnumerator1")
  (set `self.ItemName` (`|FormatText` "{Mag} Ammo" (`KismetTextLibrary.Conv_NameToText` (`self.Name`))))
  (`self.DataTable`)
  (`StaticMeshComponent.SetStaticMesh` (`self.Item_Static`) (`self.Item_Mesh`)))