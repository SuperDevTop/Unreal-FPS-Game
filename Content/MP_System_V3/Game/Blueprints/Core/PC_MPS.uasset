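; Player controller for the MPS multiplayer shooter that manages each player's UI, saved settings, input state and session exit.
; On BeginPlay it creates menu, scoreboard and countdown widgets, then loads settings, loadout and player data from the GameInstance, passing loadout and name through server events.
; Client events drive the HUD, hit feedback, kill info and pause menu, which toggles pawn input.
; Disconnecting destroys weapons and the session before loading the main menu.
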(event `self.ReceiveBeginPlay`
  ;[0.3005 0.3005 0.3005] Event Begin Play
  (`self.Client_ClearUI`)
  (`self.Client_LevelWidget`)
  (`self.Client_Scoreboard`)
  (`self.Client_Countdown`)
  (`self.RefreshSettings` false)
  (`self.RefreshLoadout`)
  (`self.LoadPlayerData`))

(event `SetEnableInput`
  ;[0.3005 0.3005 0.3005] Enable Input
  (`self.EnableInput` (`self.K2_GetPawn`) self)
  (set `self.bShowMouseCursor` false)
  (`WidgetBlueprintLibrary.SetInputMode_GameOnly` self)
  (`/Game/MP_System_V3/Game/Blueprints/Core/BP_MPS_Master.SetMovement` (`/Game/MP_System_V3/Game/Blueprints/Core/FL_MPS.Player_MPS`) "MOVE_Walking")
  (set `/Game/MP_System_V3/Game/Blueprints/Core/BP_MPS_Master.Disable_Input` false (`/Game/MP_System_V3/Game/Blueprints/Core/FL_MPS.Player_MPS`))
  (set `/Game/MP_System_V3/Game/Blueprints/Core/PS_MPS.IsDead?` false (cast `/Game/MP_System_V3/Game/Blueprints/Core/PS_MPS` (`self.PlayerState`) :!pure true)))

(event `StopInput`
  (bind _player_mps (`/Game/MP_System_V3/Game/Blueprints/Core/FL_MPS.Player_MPS`))
  ;[0.3005 0.3005 0.3005] Stop Input
  (`/Game/MP_System_V3/Game/Blueprints/Core/BP_MPS_Master.EndSprint` _player_mps false)
  (set `/Game/MP_System_V3/Game/Blueprints/Core/BP_MPS_Master.Disable_Input` true _player_mps)
  (set `/Game/MP_System_V3/Game/Blueprints/Core/BP_MPS_Master.MoveRight` 0.0 _player_mps)
  (set `/Game/MP_System_V3/Game/Blueprints/Core/BP_MPS_Master.MoveForward` 0.0 _player_mps))

(event `Svr_Loadout`
  (params (Loadout :type "Array of /Game/MP_System_V3/Game/Blueprints/Core/BP_Weapon_Master Class Reference") (WeaponID :type "Array of Integer") (SaveSlotID :type "Array of String"))
  ;[0.3005 0.3005 0.3005] Inform Server about Clients Loadout
  (set `self.Loadout` Loadout)
  (set `self.WeaponID` WeaponID)
  (set `self.Save Slot ID` SaveSlotID))

(event `Disconnect`
  ;[0.3005 0.3005 0.3005] Disconnect & End
  (for _array_element (`/Game/MP_System_V3/Game/Blueprints/Core/BP_MPS_Master.Weapons` (cast `/Game/MP_System_V3/Game/Blueprints/Core/BP_MPS_Master` (`self.K2_GetPawn` self) :!pure true))
    (`self.SVR_DestroyWeapons` _array_element))
  (`KismetSystemLibrary.Delay` 0.2)
  (`/Game/MP_System_V3/Game/Blueprints/Widgets/W_Scoreboard.RemovePlayer` (`self.W_Scoreboard`) (cast `/Game/MP_System_V3/Game/Blueprints/Core/PS_MPS` (`self.PlayerState`) :!pure true))
  (`DestroySessionCallbackProxy.DestroySession` self
    (:`OnSuccess`
      _)
    (:`OnFailure`
      _))
  (`/Game/MP_System_V3/Game/Blueprints/Core/GI_MPS.Load_MainMenu` (`/Game/MP_System_V3/Game/Blueprints/Core/FL_MPS.GameInstance_MPS`)))

(event `Svr_SetName`
  (params (Name :type Text))
  ;[0.3005 0.3005 0.3005] Override Name Replicated (only if no Steam account is linked)
)

(event `Svr_DestroyWeapons`
  (params (Weapon :type "/Game/MP_System_V3/Game/Blueprints/Core/BP_Weapon_Master Object Reference"))
  ;[0.3005 0.3005 0.3005] Disconnect & End
  (`/Engine/EditorBlueprintResources/StandardMacros.IsValid` Weapon
    (:`Is Valid`
      (`self.K2_DestroyActor` Weapon))))

(event `RefreshSettings`
  (params (`IsControllerBusy?` :type Boolean))
  ;[0.3005 0.3005 0.3005] Load / Reload Game Settings
  (set `self.IsControllerBusy?` `IsControllerBusy?`)
  (`self.LoadSettings`))

(event `EnableMovement`
  (bind _gamestate (`/Game/MP_System_V3/Game/Blueprints/Core/FL_MPS.GameState_MPS`))
  ;[0.3005 0.3005 0.3005] Enable Player Movement
  (`/Engine/EditorBlueprintResources/StandardMacros.IsValid` _gamestate
    (:`Is Valid`
      (add `/Game/MP_System_V3/Game/Blueprints/Core/GS_MPS.Dispatch_Match` _gamestate (delegate `Dispatch_StartMovement`)))))

(event `Dispatch_StartMovement`
  (bind _player_mps (`/Game/MP_System_V3/Game/Blueprints/Core/FL_MPS.Player_MPS`))
  ;[0.3005 0.3005 0.3005] Enable Player Movement
  (bind _asps_mps (cast `/Game/MP_System_V3/Game/Blueprints/Core/PS_MPS` (`self.PlayerState`))
    (:`then`
      (set `/Game/MP_System_V3/Game/Blueprints/Core/PS_MPS.IsDead?` false _asps_mps))
    (:`CastFailed`
      _))
  (`/Game/MP_System_V3/Game/Blueprints/Core/BP_MPS_Master.SetMovement` _player_mps "MOVE_Walking")
  (set `/Game/MP_System_V3/Game/Blueprints/Core/BP_MPS_Master.Disable_Input` false _player_mps)
  (`/Game/MP_System_V3/Game/Blueprints/Core/BP_MPS_Master.ReadyUp` _player_mps true)
  (if (`/Game/MP_System_V3/Game/Blueprints/Core/BP_MPS_Master.HoldSprint` _player_mps)
    (`/Game/MP_System_V3/Game/Blueprints/Core/BP_MPS_Master.StartSprint` _player_mps)))

(event `RefreshLoadout`
  ;[0.3005 0.3005 0.3005] Load / Reload Loadout
  (bind (_loadout _id _saveslotid) (`/Game/MP_System_V3/Game/Blueprints/Core/GI_MPS.LoadLoadout` (`/Game/MP_System_V3/Game/Blueprints/Core/FL_MPS.GameInstance_MPS`)))
  (`self.Svr_Loadout` _loadout _id _saveslotid))

(event `Client_IsInMenu`
  ;[0.3005 0.3005 0.3005] Get Out of Menu to Activate Pawn
  (set `self.IsInMenu?` false))

(event `Reset_ReadyState`
  ;[0.3005 0.3005 0.3005] Reset Ready State
  (set `self.IsControllerBusy?` true)
  (`KismetSystemLibrary.Delay` 0.2)
  (set `self.IsControllerBusy?` false))

(event `DisconnectAll`
  (bind _player_mps (`/Game/MP_System_V3/Game/Blueprints/Core/FL_MPS.Player_MPS`))
  ;[0.3005 0.3005 0.3005] End Session for All
  (`self.Client_ClearUI`)
  (bind _returnvalue (`|CreateWidget` "/Game/MP_System_V3/Game/Blueprints/Widgets/W_Scoreboard.W_Scoreboard_C"))
  (`/Game/MP_System_V3/Game/Blueprints/Widgets/W_Scoreboard.EndSession` _returnvalue (`self.PlayerID`))
  (`UserWidget.AddToViewport` _returnvalue 0)
  (`self.DisableInput` _player_mps self)
  (`/Game/MP_System_V3/Game/Blueprints/Core/BP_MPS_Master.SetMovement` _player_mps "MOVE_None")
  (`KismetSystemLibrary.Delay` 0.2)
  (set `/Game/MP_System_V3/Game/Blueprints/Core/BP_MPS_Master.MoveForward` 0.0 _player_mps)
  (set `/Game/MP_System_V3/Game/Blueprints/Core/BP_MPS_Master.MoveRight` 0.0 _player_mps)
  (`KismetSystemLibrary.Delay` 9.0)
  (`self.Disconnect`)
  (`/Game/MP_System_V3/Game/Blueprints/Core/GI_MPS.EndSession` (`/Game/MP_System_V3/Game/Blueprints/Core/FL_MPS.GameInstance_MPS`) self))

(event `Client_Countdown`
  ;[0.3005 0.3005 0.3005] Coutndown Widget
  (bind _returnvalue (`|CreateWidget` "/Game/MP_System_V3/Game/Blueprints/Widgets/W_Countdown.W_Countdown_C"))
  (`UserWidget.AddToViewport` _returnvalue 0))

(event `Client_HUD`
  (params (MPS :type "/Game/MP_System_V3/Game/Blueprints/Core/BP_MPS_Master Object Reference"))
  ;[0.3005 0.3005 0.3005] HUD
  (`|ExecutionSequence`
    (:`then_0`
      (`/Engine/EditorBlueprintResources/StandardMacros.DoOnce` false :!label _label
        (:`Completed`
          (bind _returnvalue (`|CreateWidget` "/Game/MP_System_V3/Game/Blueprints/Widgets/W_HUD.W_HUD_C" null MPS))
          (bind _output_get (set `self.W_HUD` _returnvalue))
          (`UserWidget.AddToViewport` _output_get 0)
          (`Widget.SetVisibility` _output_get "Collapsed"))))
    (:`then_1`
      (bind _w_ingamemenu (`self.W_InGameMenu`)
        (:`then`
          (if (not (`Widget.IsVisible` _w_ingamemenu))
            (`Widget.SetVisibility` (`self.W_HUD`) "Visible")))
        (:`else`)))))

(event `Client_ResetHUD`
  ;[0.3005 0.3005 0.3005] HUD
  (goto _label :!via `Reset`))

(event `Client_HitWheel`
  (params (DamageDealer :type "Actor Object Reference"))
  ;[0.3005 0.3005 0.3005] Hit Wheel
  (bind _returnvalue (`|CreateWidget` "/Game/MP_System_V3/Game/Blueprints/Widgets/W_HitWheel.W_HitWheel_C" null DamageDealer))
  (`UserWidget.AddToViewport` _returnvalue 0))

(event `Client_Hitmarker`
  (params (Health :type "Float (double-precision)"))
  ;[0.3005 0.3005 0.3005] HUD
  ;;[0.3005 0.3005 0.3005] Hitmarker
  (`/Game/MP_System_V3/Game/Blueprints/Widgets/W_HUD.Hit` (`self.W_HUD`) Health))

(event `Client_Damaged`
  (params (Health :type "Float (double-precision)"))
  (bind _w_hud (`self.W_HUD`))
  (bind _asbp_mps_master (cast `/Game/MP_System_V3/Game/Blueprints/Core/BP_MPS_Master` (`self.K2_GetPawn`) :!pure true))
  ;[0.3005 0.3005 0.3005] HUD
  ;;[0.3005 0.3005 0.3005] Damage Screen
  (`/Game/MP_System_V3/Game/Blueprints/Core/BC_CameraShake.SimpleCameraShake` (`/Game/MP_System_V3/Game/Blueprints/Core/BP_MPS_Master.BC_CameraShake` _asbp_mps_master) "/Game/MP_System_V3/Game/Blueprints/CameraShake/CS_Medium.CS_Medium_C" 6.0 _asbp_mps_master)
  (`/Engine/EditorBlueprintResources/StandardMacros.IsValid` _w_hud
    (:`Is Valid`
      (`/Game/MP_System_V3/Game/Blueprints/Widgets/W_HUD.Damaged` _w_hud Health))))

(event `Client_FPSCounter`
  ;[0.3005 0.3005 0.3005] FPS Counter
  (`/Engine/EditorBlueprintResources/StandardMacros.DoOnce` false :!label _label_2
    (:`Completed`
      (bind _returnvalue (`|CreateWidget` "/Game/MP_System_V3/Game/Blueprints/Widgets/W_FPS_Counter.W_FPS_Counter_C"))
      (`UserWidget.AddToViewport` _returnvalue 0))))

(event `Client_NoFPSCounter`
  ;[0.3005 0.3005 0.3005] FPS Counter
  (`/Engine/EditorBlueprintResources/StandardMacros.IsValid` (stale `Client_FPSCounter` _returnvalue)
    (:`Is Valid`
      (`Widget.RemoveFromParent` (stale `Client_FPSCounter` _returnvalue))
      (goto _label_2 :!via `Reset`))))

(event `Client_LevelWidget`
  ;[0.3005 0.3005 0.3005] Pause Widget
  (`|ExecutionSequence` :!label _label_3
    (:`then_0`
      (`/Engine/EditorBlueprintResources/StandardMacros.DoOnce` false
        (:`Completed`
          (bind _returnvalue (`|CreateWidget` "/Game/MP_System_V3/Game/Blueprints/Widgets/W_InGameMenu.W_InGameMenu_C" self))
          (bind _output_get (set `self.W_InGameMenu` _returnvalue))
          (`UserWidget.AddToViewport` _output_get 0))))
    (:`then_1`
      (set `self.bShowMouseCursor` true)
      (`WidgetBlueprintLibrary.SetInputMode_GameAndUIEx` self (`self.W_InGameMenu`) "DoNotLock" false)
      (`self.DisableInput` (`self.K2_GetPawn`) self)
      (`/Game/MP_System_V3/Game/Blueprints/Widgets/W_InGameMenu.FadeIn` (`self.W_InGameMenu`))
      (`self.StopInput`)
      (set `self.IsInMenu?` true))))

(event `Client_PauseWidget`
  (bind _w_ingamemenu (`self.W_InGameMenu`))
  ;[0.3005 0.3005 0.3005] Pause Widget
  (if (not (`Widget.GetIsEnabled` _w_ingamemenu))
    (`Widget.SetIsEnabled` _w_ingamemenu true)
    (goto _label_3)))

(event `Client_RemovePauseWidget`
  ;[0.3005 0.3005 0.3005] Pause Widget
  (`/Game/MP_System_V3/Game/Blueprints/Widgets/W_InGameMenu.FadeOut` (`self.W_InGameMenu`))
  (`self.SetEnableInput`)
  (set `self.IsInMenu?` false))

(event `InputAction|Escape`
  (params (Key :type "Key Structure"))
  ;[0.3005 0.3005 0.3005] Pause Widget
  ;;[0.3005 0.3005 0.3005] Activate / Deactivate Pause Menu
  (:`Pressed`
    (if (and (`Widget.GetIsEnabled` (`self.W_InGameMenu`)) (`/Game/MP_System_V3/Game/Blueprints/Core/BP_MPS_Master.IsReady?` (`/Game/MP_System_V3/Game/Blueprints/Core/FL_MPS.Player_MPS`))) :!label _label_4
      (`self.Client_RemovePauseWidget`)
      (`self.Client_RedrawHUD`)
      (else
        (`self.Client_PauseWidget`)))))

(event `Key|P`
  (params (Key :type "Key Structure"))
  ;[0.3005 0.3005 0.3005] Pause Widget
  ;;[0.3005 0.3005 0.3005] Activate / Deactivate Pause Menu
  ;;;[1 0.8725 0.3209] For Editor
  (:`Pressed`
    (goto _label_4)))

(event `Key|Tab`
  (params (Key :type "Key Structure"))
  (bind _w_scoreboard (`self.W_Scoreboard`))
  (bind _w_scoreboard_2 (`self.W_Scoreboard`))
  ;[0.3005 0.3005 0.3005] Tab to Check Scoreboard
  (:`Pressed`
    (if (`/Game/MP_System_V3/Game/Blueprints/Core/BP_MPS_Master.IsReady?` (`/Game/MP_System_V3/Game/Blueprints/Core/FL_MPS.Player_MPS`))
      (`Widget.SetVisibility` _w_scoreboard "Visible")
      (`/Game/MP_System_V3/Game/Blueprints/Widgets/W_Scoreboard.UpdateOrder` _w_scoreboard (`self.PlayerID`))))
  (:`Released`
    (`/Engine/EditorBlueprintResources/StandardMacros.IsValid` _w_scoreboard_2
      (:`Is Valid`
        (`Widget.SetVisibility` _w_scoreboard_2 "Collapsed")
        (`PanelWidget.ClearChildren` (`/Game/MP_System_V3/Game/Blueprints/Widgets/W_Scoreboard.Players` _w_scoreboard_2))))))

(event `Client_Scoreboard`
  ;[0.3005 0.3005 0.3005] Tab to Check Scoreboard
  (bind _returnvalue (`|CreateWidget` "/Game/MP_System_V3/Game/Blueprints/Widgets/W_Scoreboard.W_Scoreboard_C"))
  (bind _output_get (set `self.W_Scoreboard` _returnvalue))
  (`UserWidget.AddToViewport` _output_get 0)
  (`Widget.SetVisibility` _output_get "Collapsed")
  (bind _playerstate (`self.PlayerState`)
    (:`then`
      (set `self.PlayerID` (`PlayerState.GetPlayerName` _playerstate)))
    (:`else`)))

(event `HideGameWidgets`
  ;[0.3005 0.3005 0.3005] Hide In Game Widgets
  (bind _w_hud (`self.W_HUD`)
    (:`then`
      (`Widget.SetVisibility` _w_hud "Collapsed"))
    (:`else`
      _))
  (bind _w_scoreboard (`self.W_Scoreboard`)
    (:`then`
      (`Widget.SetVisibility` _w_scoreboard "Collapsed"))
    (:`else`
      _))
  (bind _w_record (`self.W_Record`)
    (:`then`
      (`Widget.SetVisibility` _w_record "Collapsed"))
    (:`else`)))

(event `Client_Kill_Info`
  (params (Name :type String) (`IsKilled?` :type Boolean))
  ;[0.3005 0.3005 0.3005] Kill Info
  (bind _returnvalue (`|CreateWidget` "/Game/MP_System_V3/Game/Blueprints/Widgets/W_KillInfo.W_KillInfo_C" null Name `IsKilled?`))
  (bind _output_get (set `self.W_KillInfo` _returnvalue))
  (`UserWidget.AddToViewport` _output_get 0))

(event `Client_ClearUI`
  ;[0.3005 0.3005 0.3005] Clear UI
  (`self.HideGameWidgets`))

(event `RecordRun`
  ;[0.3005 0.3005 0.3005] Record Run Widget
  (bind _returnvalue (`|CreateWidget` "/Game/MP_System_V3/Game/Blueprints/Widgets/W_Record.W_Record_C"))
  (bind _output_get (set `self.W_Record` _returnvalue))
  (`UserWidget.AddToViewport` _output_get 0))

(event `Client_RedrawHUD`
  ;[0.3005 0.3005 0.3005] Redraw HUD
  (`self.Client_HUD` (`/Game/MP_System_V3/Game/Blueprints/Core/FL_MPS.Player_MPS`))
  (if (`self.IsRecordingRun?`)
    (`self.RecordRun`)))

(event `Client_AimPose`
  ;[1 0.8725 0.3209] Aim Pose (For Development Only)
  (bind _returnvalue (`|CreateWidget` "/Game/MP_System_V3/Game/Blueprints/Widgets/W_AimPoseInfo.W_AimPoseInfo_C"))
  (`UserWidget.AddToViewport` _returnvalue 0))

(event `Key|Zero`
  (params (Key :type "Key Structure"))
  ;[1 0.8725 0.3209] Aim Pose (For Development Only)
  (:`Pressed`
    (`self.Client_AimPose`)))

(fn `LoadPlayerData`
  (bind _playerdata (`/Game/MP_System_V3/Game/Blueprints/Core/GI_MPS.LoadPlayerSettings` (`/Game/MP_System_V3/Game/Blueprints/Core/FL_MPS.GameInstance_MPS`)))
  (set `self.Player_MainMesh` (break `/Game/MP_System_V3/Game/Blueprints/Structs/ST_PlayerData` _playerdata))
  (set `self.Player_SecondaryMesh` (`.SecondaryMesh_4_EE5E310D4FF6D0F440F23180B0FCE4A2` (break `/Game/MP_System_V3/Game/Blueprints/Structs/ST_PlayerData` _playerdata)))
  (set `self.Player_MainMaterial` (`.MainMaterial_8_0223858B4BCCE2E96CB55D8CD157C85C` (break `/Game/MP_System_V3/Game/Blueprints/Structs/ST_PlayerData` _playerdata))))

(fn `LoadSettings`
  (bind (_playernames _settings) (`/Game/MP_System_V3/Game/Blueprints/Core/GI_MPS.LoadSettings` (`/Game/MP_System_V3/Game/Blueprints/Core/FL_MPS.GameInstance_MPS`)))
  (bind ((`Name_39_71BF07254DEF36CDDC241192B0ACD5F5` _name) (`ShowFPS_33_BF6D12AA492BFC8242DEC2B1CC159588` _showfps) (`UseBlur_48_4DADECF84EC0C292E30ADCBE0B01087D` _useblur) (`FOV_43_ACB5AE884A48FA208A88CA98A188D77B` _fov) (`MouseSensitivity_46_92255ECA486A9A57E112EF9CD5E9458B` _mousesensitivity) (`UseInterruptedReload_69_33F24C9945583C5880056EBEB9840C56` _useinterruptedreload) (`SprintInterruptsReload_70_DEB83A864345DED32095F389747291C4` _sprintinterruptsreload) (`FirstDrawAfterEverySpawn_79_39D13D3F4A52992ADE8230B15F336DBB` _firstdrawaftereveryspawn)) (break `/Game/MP_System_V3/Game/Blueprints/Structs/ST_SaveSettings` _settings))
  (`self.Svr_SetName` _name)
  (set `self.FieldOfView` _fov)
  (set `self.MouseSensitivity` _mousesensitivity)
  (set `self.UseBlur?` _useblur)
  (set `self.UseInterruptedReload?` _useinterruptedreload)
  (set `self.SprintInterruptsReload?` _sprintinterruptsreload)
  (set `self.FirstDrawEverySpawn` _firstdrawaftereveryspawn)
  (if _showfps
    (`self.Client_FPSCounter`)
    (else
      (`self.Client_NoFPSCounter`))))

(fn `OnRep_IsMenuActive?`)

(fn `UserConstructionScript`)