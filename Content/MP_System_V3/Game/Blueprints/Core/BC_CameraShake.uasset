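; Character component on BP_MPS_Master that plays camera shakes, only for the locally controlled player.
; A looping timer plays walk or sprint shakes chosen and scaled by owner speed, skipping them while jumping.
; A bound TPC shake event replaces the base shake at a given intensity.
; Callable events play a supplied shake or pick one by type, from light to explosion.
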(event `self.ReceiveBeginPlay`
  ;[0.3005 0.3005 0.3005] Construct and Loop for Movement
  (bind _asbp_mps_master (cast `/Game/MP_System_V3/Game/Blueprints/Core/BP_MPS_Master` (`self.GetOwner`)))
  (set `self.MPS` _asbp_mps_master)
  (`KismetSystemLibrary.K2_SetTimer` null "Movement" 0.52 true)
  (add `self.TPC_Shake` (delegate `Start_TPC_Shake`)))

(event `Start_TPC_Shake` :!signature `self.TPC_Shake`
  (params (ShakeIntensity :type "Float (double-precision)"))
  ;[0.3005 0.3005 0.3005] Construct and Loop for Movement
  (`self.StopAllCameraShakesOfType` "/Game/MP_System_V3/Game/Blueprints/CameraShake/CS_Base.CS_Base_C")
  (`self.SimpleCameraShake` "/Game/MP_System_V3/Game/Blueprints/CameraShake/CS_Base.CS_Base_C" ShakeIntensity (`self.MPS`)))

(event `SimpleCameraShake`
  (params (Effect :type "CameraShakeBase Class Reference") (Scale :type "Float (double-precision)") (Owner :type "Pawn Object Reference"))
  ;[0.3005 0.3005 0.3005] Simple Camera Shake called in MPS Master
  (if (`Pawn.IsLocallyControlled` Owner)
    (`self.StartCameraShake` Effect Scale)))

(event `SwitchCameraShakes`
  (params (Scale :type "Float (double-precision)") (Type :type Name) (Target :type "Pawn Object Reference"))
  (bind _number (`self.Number`))
  ;[0.3005 0.3005 0.3005] Selection of Camera Shakes
  (if (`BlueprintMapLibrary.Map_Contains` _number Type)
    (if (`Pawn.IsLocallyControlled` Target)
      (`self.StartCameraShake` (select `int` (`BlueprintMapLibrary.Map_Find` _number Type) :`0` "/Game/MP_System_V3/Game/Blueprints/CameraShake/CS_Light.CS_Light_C" :`1` "/Game/MP_System_V3/Game/Blueprints/CameraShake/CS_Medium.CS_Medium_C" :`2` "/Game/MP_System_V3/Game/Blueprints/CameraShake/CS_Strong.CS_Strong_C" :`3` "/Game/MP_System_V3/Game/Blueprints/CameraShake/CS_Strongest.CS_Strongest_C" :`4` "/Game/MP_System_V3/Game/Blueprints/CameraShake/CS_Explosion.CS_Explosion_C" :!type "CameraShakeBase Class Reference") Scale))))

(fn `Movement`
  (bind _mps (`self.MPS`))
  (bind _returnvalue (`KismetMathLibrary.VSize` (`Actor.GetVelocity` _mps)))
  (if (not (`/Game/MP_System_V3/Game/Blueprints/Core/BP_MPS_Master.IsJumping?` _mps))
    (`self.SimpleCameraShake` (select `bool` (> _returnvalue 400.0) :`false` "/Game/MP_System_V3/Game/Blueprints/CameraShake/CS_Walk.CS_Walk_C" :`true` "/Game/MP_System_V3/Game/Blueprints/CameraShake/CS_Sprint.CS_Sprint_C" :!type "CameraShakeBase Class Reference") (`KismetMathLibrary.NormalizeToRange` _returnvalue 0.0 300.0) (`self.MPS`))))