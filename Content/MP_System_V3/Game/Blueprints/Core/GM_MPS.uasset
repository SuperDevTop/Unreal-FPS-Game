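; GM_MPS is the game mode for a multiplayer system, handling player spawning and respawning.
; Each joining controller is tracked in ConnectedControllers, given a CBP_MPS_A pawn at a random PlayerStart and possessed, then CallNewPlayer fires.
; RespawnPlayer finds the controller of a given pawn, unpossesses it, spawns a fresh pawn and calls Alive on its PS_MPS player state.
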(event `self.HandleStartingNewPlayer`
  (params (NewPlayer :type "PlayerController Object Reference"))
  ;[0.3005 0.3005 0.3005] On Joining the Match
  (bind _output_get (set `self.NewPlayerController` NewPlayer))
  (`KismetArrayLibrary.Array_AddUnique` (`self.ConnectedControllers`) _output_get)
  (`self.SpawnPlayers` "/Script/Engine.PlayerStart" "/Game/MP_System_V3/Game/Blueprints/CBP_MPS_A.CBP_MPS_A_C" _output_get)
  (`self.NewPlayer`))

(fn `RespawnPlayer`
  (params (Player :type "Character Object Reference") (PlayerState :type "PlayerState Object Reference"))
  (locals (Controller :type "Controller Object Reference"))
  (for _array_element (`self.ConnectedControllers`)
    (if (== (`Controller.K2_GetPawn` _array_element) Player)
      (bind _output_get (set `local.Controller` _array_element))
      (`Controller.UnPossess` _output_get)
      (`self.SpawnPlayers` "/Script/Engine.PlayerStart" "/Game/MP_System_V3/Game/Blueprints/CBP_MPS_A.CBP_MPS_A_C" (`local.Controller`))
      (bind _asps_mps (cast `/Game/MP_System_V3/Game/Blueprints/Core/PS_MPS` PlayerState))
      (`/Game/MP_System_V3/Game/Blueprints/Core/PS_MPS.Alive` _asps_mps))))

(fn `SpawnPlayers`
  (params (SpawnPoint :type "Actor Class Reference") (Player :type "/Game/MP_System_V3/Game/Blueprints/Core/BP_MPS_Master Class Reference") (Controller :type "Controller Object Reference"))
  (bind _outactors (`GameplayStatics.GetAllActorsOfClass` SpawnPoint))
  (bind _returnvalue (`|SpawnActorFromClass` Player (`self.GetTransform` (`|GetArrayItem` _outactors (`KismetMathLibrary.RandomInteger` (`KismetArrayLibrary.Array_Length` _outactors)))) "AdjustIfPossibleButAlwaysSpawn" "OverrideRootScale" Controller null))
  (`/Engine/EditorBlueprintResources/StandardMacros.IsValid` _returnvalue
    (:`Is Valid`
      (`Controller.Possess` Controller _returnvalue))))

(fn `UserConstructionScript`)