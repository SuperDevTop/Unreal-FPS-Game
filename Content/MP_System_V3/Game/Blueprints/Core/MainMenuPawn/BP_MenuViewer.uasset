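; Main menu pawn that showcases the player's character and weapon and provides an item viewer.
; BeginPlay overwrites saved player settings with a hardcoded look, then builds a hidden body with a master-posed vest.
; Spawning reveals it with the first loadout weapon or a default sniper, setting left-hand grip offsets.
; The viewer centers items on an arrow for right-mouse rotation and adjusts focal distance, while a timeline fades in suit glows.
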(event `self.ReceiveBeginPlay`
  (bind (_returnvalue_location _returnvalue_rotation _returnvalue_scale) (`KismetMathLibrary.BreakTransform` (`self.GetTransform`)))
  ;[0.3005 0.3005 0.3005] Set Up Character
  (bind _aspc_menu (cast `/Game/MP_System_V3/Game/Blueprints/Core/MainMenuPawn/PC_Menu` (`GameplayStatics.GetPlayerController` 0))
    (:`then`
      (add `/Game/MP_System_V3/Game/Blueprints/Core/MainMenuPawn/PC_Menu.Skip` _aspc_menu (delegate `Skip`)))
    (:`CastFailed`
      _))
  (`/Game/MP_System_V3/Game/Blueprints/Core/GI_MPS.LoadPlayerSettings` (`/Game/MP_System_V3/Game/Blueprints/Core/FL_MPS.GameInstance_MPS`))
  (`/Game/MP_System_V3/Game/Blueprints/Core/GI_MPS.SavePlayerSettings` (`/Game/MP_System_V3/Game/Blueprints/Core/FL_MPS.GameInstance_MPS`) (make `/Game/MP_System_V3/Game/Blueprints/Structs/ST_PlayerData` "/Game/MP_System_V3/Game/Characters/Mannequin/Mesh/MPS_Player.MPS_Player" "/Game/MP_System_V3/Game/Characters/Accessories/TacticalVest/Tactical_V2.Tactical_V2" "/Game/MP_System_V3/Game/Characters/Mannequin/Materials/MI_MPS.MI_MPS"))
  (bind _returnvalue (`AddComponent|NODE_AddSkeletalMeshComponent-1` :`RelativeTransform` (`KismetMathLibrary.MakeTransform` (+ _returnvalue_location (75.0 0.0 -145.0)) (struct :`Yaw` 65.0) _returnvalue_scale)))
  (set `self.Character` _returnvalue)
  (bind _returnvalue_2 (`AddComponent|NODE_AddSkeletalMeshComponent-4`))
  (set `self.Vest` _returnvalue_2)
  (`self.DefineMesh`)
  (`self.SecureAttachment`))

(event `Skip`
  ;[0.3005 0.3005 0.3005] Set Up Character
  (`KismetSystemLibrary.Delay` 1.0)
  (`self.SpawnCharacter`))

(event `ShowcaseWeapon`
  (bind _returnvalue (`SceneComponent.GetSocketTransform` (`self.Character`) "Weapon" "RTS_World"))
  (bind _modifygrip (`/Game/MP_System_V3/Game/Blueprints/Core/BP_Weapon_Master.ModifyGrip` (`self.Weapon`)))
  (bind _value (`BlueprintMapLibrary.Map_Find` (`self.List`) (`KismetStringLibrary.LeftChop` (`self.ID`) 9)))
  ;[0.3005 0.3005 0.3005] Get Active Weapon or Default to Sniper Rifle
  (bind _weapon (`self.Weapon`)
    (:`then`
      (`self.K2_DestroyActor` _weapon))
    (:`else`
      _))
  (bind (_loadout _id _saveslotid) (`/Game/MP_System_V3/Game/Blueprints/Core/GI_MPS.LoadLoadout` (`/Game/MP_System_V3/Game/Blueprints/Core/FL_MPS.GameInstance_MPS`)))
  (bind _output (`|GetArrayItem` _loadout))
  (if (== _output null)
    (bind _output_get (set `self.ID` "Sniper_00000000"))
    (bind _returnvalue_2 (`|SpawnActorFromClass` "/Game/MP_System_V3/Game/Weapons/Primary/Sniper/BP_Sniper.BP_Sniper_C" _returnvalue "Undefined" "OverrideRootScale" null true 0.0 _output_get "NewEnumerator4" "NewEnumerator5" "NewEnumerator5" "NewEnumerator5" null))
    (set `self.Weapon` _returnvalue_2)
    (else
      (bind _output_get_2 (set `self.ID` (`|GetArrayItem` _saveslotid (`|GetArrayItem` _id))))
      (bind _returnvalue_3 (`|SpawnActorFromClass` _output _returnvalue "Undefined" "OverrideRootScale" null false 0.0 _output_get_2 "NewEnumerator0" "NewEnumerator5" "NewEnumerator5" "NewEnumerator5" null))
      (set `self.Weapon` _returnvalue_3)))
  (`self.K2_AttachToComponent` (`self.Weapon`) (`self.Character`) "Weapon" "SnapToTarget" "SnapToTarget" "KeepRelative" true)
  (set `self.LH_Offset` (select `int` _value :`0` (select `bool` _modifygrip :`false` (-28.917 17.931 0.494) :`true` (-35.735001 24.563 -6.385) :!type "Vector Structure") :`1` (-43.653 26.191999 -2.016) :`2` (-33.527 17.368 1.433)))
  (set `self.LH_Rotation` (select `int` _value :`0` (select `bool` _modifygrip :`false` (struct :`Pitch` -28.556999 :`Yaw` -167.554001 :`Roll` 132.785995) :`true` (struct :`Pitch` -4.065 :`Yaw` -137.957001 :`Roll` -176.649002) :!type "Rotator Structure") :`1` (struct :`Pitch` -1.715 :`Yaw` -140.110001 :`Roll` -175.261993) :`2` (struct :`Pitch` -11.236 :`Yaw` -157.052994 :`Roll` 105.612999))))

(event `Key|RightMouseButton`
  (params (Key :type "Key Structure"))
  ;[0.3005 0.3005 0.3005] Can Turn
  (:`Pressed`
    (set `self.CanTurn?` true))
  (:`Released`
    (set `self.CanTurn?` false)))

(event `GetViewerObject`
  (params (Item :type "/Game/MP_System_V3/Game/Blueprints/Core/BP_InteractionMaster Object Reference") (Length :type "Float (double-precision)"))
  (bind _length (`self.Length`))
  ;[0.3005 0.3005 0.3005] Retrieve Item and Center it
  (bind _output_get (set `self.Item` (`/Game/MP_System_V3/Game/Blueprints/Core/BP_InteractionMaster.Item` Item)))
  (set `self.Length` Length)
  (set `self.StoredTransform` (`SceneComponent.K2_GetComponentToWorld` _output_get))
  (`SceneComponent.K2_AttachToComponent` _output_get (`self.Arrow`) "None" "SnapToTarget" "SnapToTarget" "KeepRelative" true)
  (bind (_returnvalue_x _returnvalue_y _returnvalue_z) (`KismetMathLibrary.BreakVector` (`SceneComponent.K2_GetComponentLocation` _output_get)))
  (bind (_returnvalue_x_2 _returnvalue_y_2 _returnvalue_z_2) (`KismetMathLibrary.BreakVector` (`SceneComponent.GetSocketLocation` _output_get "Center")))
  (`SceneComponent.K2_AddWorldOffset` _output_get (`KismetMathLibrary.MakeVector` (- _returnvalue_x _returnvalue_x_2) (- _returnvalue_y _returnvalue_y_2) (- _returnvalue_z _returnvalue_z_2)) false false)
  (bind _aspc_menu (cast `/Game/MP_System_V3/Game/Blueprints/Core/MainMenuPawn/PC_Menu` (`GameplayStatics.GetPlayerController` 0)))
  (`WidgetBlueprintLibrary.SetInputMode_GameOnly` _aspc_menu)
  (set `self.IsViewer?` true)
  (set `self.CanTurn?` false)
  (`KismetSystemLibrary.K2_SetTimer` null "Rotation" 0.01 true)
  (`SceneComponent.K2_SetWorldTransform` (`self.Arrow`) (`KismetMathLibrary.MakeTransform` (`KismetMathLibrary.MakeVector` (+ (* _length -0.5) 10.0))) false false)
  (setmembers `PostProcessSettings` :`StructRef` (`CameraComponent.PostProcessSettings` (`self.Camera`)) :`DepthOfFieldFocalDistance` (`KismetMathLibrary.FClamp` (`KismetMathLibrary.Abs` (+ _length 10.0)) 40.0 100.0)))

(event `TurnLightsOn`
  (bind _character (`self.Character`))
  (bind _character_2 (`self.Character`))
  ;[0.3005 0.3005 0.3005] Set Lights
  (bind _asanim_bp_menu (cast `/Game/MP_System_V3/Game/Blueprints/Core/MainMenuPawn/AnimBP_Menu` (`SkeletalMeshComponent.GetAnimInstance` _character))
    (:`then`
      (set `/Game/MP_System_V3/Game/Blueprints/Core/MainMenuPawn/AnimBP_Menu.Additive` 0.0 _asanim_bp_menu))
    (:`CastFailed`
      _))
  (if (== (`PrimitiveComponent.GetMaterial` _character 0) "/Game/MP_System_V3/Game/Characters/Mannequin/Materials/MI_MPS.MI_MPS")
    (bind _returnvalue (`PrimitiveComponent.CreateDynamicMaterialInstance` _character_2 0 (`PrimitiveComponent.GetMaterial` _character_2 0) "None"))
    (`SceneComponent.SetVisibility` (`self.ParticleSystem`) true false)
    (bind (_direction _lightstrength) (`Timeline|SetLights` :!via `PlayFromStart` :!label _label)
      (:`Update`
        (`MaterialInstanceDynamic.SetScalarParameterValue` _returnvalue "EmissiveAmount" (* _lightstrength 60.0))
        (`self.GlowAmount` (`self.Glow_R`) _lightstrength)
        (`self.GlowAmount` (`self.Glow_R1`) _lightstrength)
        (`self.GlowAmount` (`self.Glow_R2`) _lightstrength)
        (`self.GlowAmount` (`self.Glow_L`) _lightstrength)
        (`self.GlowAmount` (`self.Glow_L1`) _lightstrength)
        (`self.GlowAmount` (`self.Glow_L2`) _lightstrength)
        (`LightComponent.SetIntensity` (`self.Light`) (* _lightstrength 5000.0))
        (`SceneComponent.SetWorldScale3D` (`self.ParticleSystem`) (`KismetMathLibrary.Conv_DoubleToVector` (`KismetMathLibrary.FClamp` (* _lightstrength 10.0))))))))

(event `TurnLightsOff`
  ;[0.3005 0.3005 0.3005] Set Lights
  (goto _label :!via `SetNewTime`))

(event `SpawnCharacter`
  ;[0.3005 0.3005 0.3005] Spawn Character with Anims
  (`/Engine/EditorBlueprintResources/StandardMacros.DoOnce` false
    (:`Completed`
      (if (not (`self.IsSpawned?`))
        (set `self.IsSpawned?` true)
        (`KismetSystemLibrary.Delay` 0.2)
        (`SceneComponent.SetHiddenInGame` (`self.Character`) false true)
        (`self.ShowcaseWeapon`)))))

(event `ExitViewer`
  ;[0.3005 0.3005 0.3005] Exit Viewer
  (`SceneComponent.K2_DetachFromComponent` (`self.Item`) "KeepRelative" "KeepRelative" "KeepRelative" true)
  (set `self.IsViewer?` false)
  (`SceneComponent.K2_SetWorldTransform` (`self.Item`) (`self.StoredTransform`) false false)
  (`SceneComponent.K2_SetWorldTransform` (`self.Arrow`) (`self.ZeroTransform`) false false)
  (setmembers `PostProcessSettings` :`StructRef` (`CameraComponent.PostProcessSettings` (`self.Camera`)) :`DepthOfFieldFocalDistance` 0.0))

(fn `DefineMesh`
  (bind _vest (`self.Vest`))
  (bind _character (`self.Character`))
  (bind _character_2 (`self.Character`))
  (bind _playerdata (`/Game/MP_System_V3/Game/Blueprints/Core/GI_MPS.LoadPlayerSettings` (`/Game/MP_System_V3/Game/Blueprints/Core/FL_MPS.GameInstance_MPS`)))
  (bind (_mainmesh _secondarymesh _mainmaterial) (break `/Game/MP_System_V3/Game/Blueprints/Structs/ST_PlayerData` _playerdata))
  (`SkinnedMeshComponent.SetSkinnedAssetAndUpdate` _character _mainmesh true)
  (`PrimitiveComponent.SetMaterial` _character 0 _mainmaterial)
  (`SkinnedMeshComponent.SetSkinnedAssetAndUpdate` _vest _secondarymesh true)
  (`SceneComponent.K2_AttachToComponent` _vest (`self.Character`) "None" "SnapToTarget" "SnapToTarget" "KeepRelative" true)
  (`SkinnedMeshComponent.SetLeaderPoseComponent` (`self.Vest`) _character_2 true)
  (`SceneComponent.SetHiddenInGame` _character_2 true true))

(fn `GlowAmount`
  (params (Target :type "PrimitiveComponent Object Reference") (Opacity :type "Float (double-precision)"))
  (bind _returnvalue (`PrimitiveComponent.CreateDynamicMaterialInstance` Target 0 (`PrimitiveComponent.GetMaterial` Target 0) "None"))
  (`MaterialInstanceDynamic.SetScalarParameterValue` _returnvalue "Opacity" (`KismetMathLibrary.FClamp` (* Opacity 20.0) 0.0 0.75))
  (`MaterialInstanceDynamic.SetScalarParameterValue` _returnvalue "Emissive" (* Opacity 100.0)))

(fn `Rotation`
  (bind _arrow (`self.Arrow`))
  (`/Engine/EditorBlueprintResources/StandardMacros.IsValid` (`self.Item`)
    (:`Is Valid`
      (if (and (`self.IsViewer?`) (`self.CanTurn?`))
        (`SceneComponent.K2_SetWorldRotation` _arrow (`KismetMathLibrary.ComposeRotators` (`SceneComponent.K2_GetComponentRotation` _arrow) (`KismetMathLibrary.MakeRotator` 0.0 (* (`self.GetInputAxisKeyValue`) 3.0) (* (`self.GetInputAxisKeyValue`) -3.0))) false false)))))

(fn `UserConstructionScript`)