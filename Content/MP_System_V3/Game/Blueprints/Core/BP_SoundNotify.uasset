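; BP_SoundNotify is an animation notify state that plays a configurable sound on a weapon for the length of the notify window.
; On begin, it casts the mesh owner to BP_Weapon_Master, sets the sound on that weapon's AudioNotify audio component, plays it, then applies pitch and volume multipliers.
; On end, it stops the same component, and both events do nothing if the owner is not a BP_Weapon_Master.
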(fn `Received_NotifyBegin`
  (params (MeshComp :type "SkeletalMeshComponent Object Reference") (Animation :type "AnimSequenceBase Object Reference") (TotalDuration :type "Float (single-precision)") (EventReference :type "AnimNotifyEventReference Structure (by ref)"))
  (returns (ReturnValue :type Boolean))
  (bind _asbp_weapon_master (cast `/Game/MP_System_V3/Game/Blueprints/Core/BP_Weapon_Master` (`ActorComponent.GetOwner` MeshComp)))
  (bind _audionotify (`/Game/MP_System_V3/Game/Blueprints/Core/BP_Weapon_Master.AudioNotify` _asbp_weapon_master))
  (`AudioComponent.SetSound` _audionotify (`self.Sound`))
  (`AudioComponent.Play` _audionotify 0.0)
  (`AudioComponent.SetPitchMultiplier` _audionotify (`self.Pitch`))
  (`AudioComponent.SetVolumeMultiplier` _audionotify (`self.Volume`))
  (return false))

(fn `Received_NotifyEnd`
  (params (MeshComp :type "SkeletalMeshComponent Object Reference") (Animation :type "AnimSequenceBase Object Reference") (EventReference :type "AnimNotifyEventReference Structure (by ref)"))
  (returns (ReturnValue :type Boolean))
  (bind _asbp_weapon_master (cast `/Game/MP_System_V3/Game/Blueprints/Core/BP_Weapon_Master` (`ActorComponent.GetOwner` MeshComp)))
  (`AudioComponent.Stop` (`/Game/MP_System_V3/Game/Blueprints/Core/BP_Weapon_Master.AudioNotify` _asbp_weapon_master))
  (return false))