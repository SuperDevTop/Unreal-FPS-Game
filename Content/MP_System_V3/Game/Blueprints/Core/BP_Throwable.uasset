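; BP_Throwable is a networked thrown explosive that detonates after a delay or when HitExplode is called.
; The server event applies radial falloff damage with a negative base value, credited to the instigator's controller, fires a radial force impulse and destroys the actor.
; A multicast event plays the explosion particles, decal, camera shake and sound.
; The construction script sets the skeletal mesh from a variable.
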(event `HitExplode`
  ;[0.3005 0.3005 0.3005] Initiate Explosion with Timer or with Hit
  (`self.Svr_Explode` :!label _label))

(event `self.ReceiveBeginPlay`
  ;[0.3005 0.3005 0.3005] Initiate Explosion with Timer or with Hit
  (`KismetSystemLibrary.Delay` (`self.ExplosionDelay`))
  (goto _label))

(event `Svr_Explode`
  (bind _returnvalue (`self.K2_GetActorLocation`))
  ;[0.3005 0.3005 0.3005] Server Explosion Damage
  (`self.MC_Explode` _returnvalue)
  (`GameplayStatics.ApplyRadialDamageWithFalloff` :`BaseDamage` -200.0 :`Origin` _returnvalue :`DamageInnerRadius` 400.0 :`DamageOuterRadius` 800.0 :`DamageFalloff` 2.0 :`DamageTypeClass` "/Engine/EngineDamageTypes/DmgTypeBP_Environmental.DmgTypeBP_Environmental_C" :`DamageCauser` null :`InstigatedByController` (cast `/Game/MP_System_V3/Game/Blueprints/Core/PC_MPS` (`self.GetInstigatorController`) :!pure true))
  (`RadialForceComponent.FireImpulse` (`self.RadialForce`))
  (`self.K2_DestroyActor`))

(event `MC_Explode`
  (params (Location :type "Vector Structure"))
  ;[0.3005 0.3005 0.3005] Multicast Explosion Effects
  (`GameplayStatics.SpawnEmitterAtLocation` "/Game/MP_System_V3/Game/Commons/Particles/P_Explosion.P_Explosion" Location (struct) (3.0 3.0 3.0))
  (`GameplayStatics.SpawnDecalAtLocation` "/Game/MP_System_V3/Game/Commons/Materials/Masters/M_BulletDecal.M_BulletDecal" (100.0 100.0 100.0) Location (struct :`Pitch` -90.0) 20.0)
  (`GameplayStatics.PlayWorldCameraShake` "/Game/MP_System_V3/Game/Blueprints/CameraShake/CS_Explosion.CS_Explosion_C" Location 0.0 2000.0 10.0 true)
  (`GameplayStatics.PlaySoundAtLocation` "/Game/MP_System_V3/Game/Sounds/Cue/Explosion_Cue.Explosion_Cue" Location (struct) 1.0 1.0 0.0 null null null null))

(fn `UserConstructionScript`
  (`SkinnedMeshComponent.SetSkinnedAssetAndUpdate` (`self.Explosive`) (`self.Mesh`) true))