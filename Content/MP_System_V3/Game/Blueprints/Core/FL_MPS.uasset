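; Blueprint function library of shared helpers for the MPS multiplayer system's core classes and widgets.
; Getters return the game instance, game mode, game state, player controller and controlled pawn, each cast to its MPS class.
; The controller and pawn lookups always use player index 0.
; Widget helpers toggle hover opacity through color tint and swap a text's typeface while keeping its other font settings.
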(fn `GameInstance_MPS`
  (returns (GameInstance :type "/Game/MP_System_V3/Game/Blueprints/Core/GI_MPS Object Reference"))
  (bind _asgi_mps (cast `/Game/MP_System_V3/Game/Blueprints/Core/GI_MPS` (`GameplayStatics.GetGameInstance` (`local.__WorldContext`))))
  (return _asgi_mps))

(fn `GameMode_MPS`
  (returns (`AsGM MPS` :type "/Game/MP_System_V3/Game/Blueprints/Core/GM_MPS Object Reference"))
  (bind _asgm_mps (cast `/Game/MP_System_V3/Game/Blueprints/Core/GM_MPS` (`GameplayStatics.GetGameMode` (`local.__WorldContext`))))
  (return _asgm_mps))

(fn `GameState_MPS`
  (returns (GameState :type "/Game/MP_System_V3/Game/Blueprints/Core/GS_MPS Object Reference"))
  (bind _asgs_mps (cast `/Game/MP_System_V3/Game/Blueprints/Core/GS_MPS` (`GameplayStatics.GetGameState` (`local.__WorldContext`))))
  (return _asgs_mps))

(fn `Player_MPS`
  (returns (Player_MPS :type "/Game/MP_System_V3/Game/Blueprints/Core/BP_MPS_Master Object Reference"))
  (bind _asbp_mps_master (cast `/Game/MP_System_V3/Game/Blueprints/Core/BP_MPS_Master` (`Controller.K2_GetPawn` (`GameplayStatics.GetPlayerController` (`local.__WorldContext`)))))
  (return _asbp_mps_master))

(fn `PlayerController_MPS`
  (returns (PlayerController :type "/Game/MP_System_V3/Game/Blueprints/Core/PC_MPS Object Reference"))
  (bind _aspc_mps (cast `/Game/MP_System_V3/Game/Blueprints/Core/PC_MPS` (`GameplayStatics.GetPlayerController` (`local.__WorldContext`))))
  (return _aspc_mps))

(fn `W_Hover`
  (params (Target :type "Button Object Reference"))
  (`Button.SetColorAndOpacity` Target (struct :`R` 1.0 :`G` 1.0 :`B` 1.0 :`A` 1.0)))

(fn `W_Typeface`
  (params (Text :type "TextBlock Object Reference") (Typeface :type Name))
  (bind (_font_fontobject _font_fontmaterial _font_outlinesettings _font_typefacefontname _font_size _font_letterspacing) (break `SlateFontInfo` (`TextBlock.Font` Text)))
  (`TextBlock.SetFont` Text (make `SlateFontInfo` _font_fontobject _font_fontmaterial _font_outlinesettings Typeface _font_size _font_letterspacing)))

(fn `W_Unhover`
  (params (Target :type "Button Object Reference"))
  (`Button.SetColorAndOpacity` Target (struct :`R` 1.0 :`G` 1.0 :`B` 1.0 :`A` 0.75)))