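; Physical bullet projectile for the MPS multiplayer shooter that detects hits with line traces rather than collision events.
; Each tick traces ahead along its velocity, starting at the weapon muzzle for a brief initial window, then from the bullet itself.
; A hit reports to the instigator's SvrLineTrace, detonates throwables, triggers bullet penetration and destroys the bullet.
; A miss starts a delayed self-destruct.
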(event `self.ReceiveBeginPlay`
  ;[0.3005 0.3005 0.3005] Switch to Bullet Trace After 0.1s
  (`KismetSystemLibrary.Delay` 0.1)
  (set `self.Pick A` true))

(event `self.ReceiveTick`
  (params (DeltaSeconds :type "Float (single-precision)"))
  (bind _returnvalue (`SceneComponent.K2_GetComponentLocation` (`self.Bullet`)))
  (bind _asbp_mps_master (cast `/Game/MP_System_V3/Game/Blueprints/Core/BP_MPS_Master` (`self.Instigator`) :!pure true))
  (bind _array (`|MakeArray` (`/Game/MP_System_V3/Game/Blueprints/Core/BP_MPS_Master.ActiveWeapon` _asbp_mps_master) _asbp_mps_master :!type "Actor Object Reference"))
  ;[0.3005 0.3005 0.3005] Line Trace at Tick Rate of 0.01s
  (bind (_outhit _returnvalue_2) (`KismetSystemLibrary.LineTraceSingle` (`KismetMathLibrary.SelectVector` _returnvalue (`SceneComponent.GetSocketLocation` (`/Game/MP_System_V3/Game/Blueprints/Core/BP_InteractionMaster.Item` (`/Game/MP_System_V3/Game/Blueprints/Core/BP_MPS_Master.ActiveWeapon` _asbp_mps_master)) "Muzzle") (`self.Pick A`)) (+ _returnvalue (* (`KismetMathLibrary.Normal` (`MovementComponent.Velocity` (`self.ProjectileMovement`))) 1000)) "TraceTypeQuery2" false _array))
  (if _returnvalue_2
    (bind (_bblockinghit _binitialoverlap _time _distance _location _impactpoint _normal _impactnormal _physmat _hitactor _hitcomponent _hitbonename _bonename _hititem _elementindex _faceindex _tracestart) (`GameplayStatics.BreakHitResult` _outhit))
    (`/Game/MP_System_V3/Game/Blueprints/Core/BP_MPS_Master.Svr_LineTrace` _asbp_mps_master (`KismetMathLibrary.Vector_Distance` _impactpoint (`self.K2_GetActorLocation` _asbp_mps_master)) _impactpoint _impactnormal (`KismetMathLibrary.GetDirectionUnitVector` _impactnormal _tracestart) _physmat _hitactor _hitbonename _outhit)
    (bind _asbp_throwable (cast `/Game/MP_System_V3/Game/Blueprints/Core/BP_Throwable` _hitactor)
      (:`then`
        (`/Game/MP_System_V3/Game/Blueprints/Core/BP_Throwable.HitExplode` _asbp_throwable))
      (:`CastFailed`
        _))
    (`/Game/MP_System_V3/Game/Blueprints/Core/BP_MPS_Master.CallBulletPenetration` _asbp_mps_master (`MovementComponent.Velocity` (`self.ProjectileMovement`)) _outhit _array)
    (`self.K2_DestroyActor`)
    (else
      (`KismetSystemLibrary.Delay` 3.0)
      (`self.K2_DestroyActor`))))

(fn `UserConstructionScript`)