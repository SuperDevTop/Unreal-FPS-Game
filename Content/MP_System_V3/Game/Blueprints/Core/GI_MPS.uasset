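; Game instance for the MPS multiplayer game that owns session flow, level travel and local save data.
; Hosts, joins and destroys sessions, opening hosted maps as listen servers, with delayed map-name checks to catch failed loads.
; Network errors, travel errors and shutdown return to the main menu.
; Separate save objects persist settings, stats and match time, loadout, and player data; saving a loadout refreshes the player controller.
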(event `self.ReceiveInit`
  ;[0.3005 0.3005 0.3005] Save / Load Settings
  (`self.LoadSettings`))

(event `Client_SaveLoadout`
  (params (Loadout :type "Array of /Game/MP_System_V3/Game/Blueprints/Core/BP_Weapon_Master Class Reference (by ref)") (ID :type "Array of Integer (by ref)") (SaveSlotID :type "Array of String"))
  ;[0.3005 0.3005 0.3005] Save / Load Settings
  (`self.SaveLoadout` Loadout ID SaveSlotID))

(event `Host_Sessions`
  (params (MaxPlayers :type Integer) (bUseLAN :type Boolean) (SessionName :type String) (MapName :type String))
  ;[0.3005 0.3005 0.3005] Host Multiplayer Session (Server)
  ;;[1 0.6702 0.1962 1 10] Create Advanced Session
  (`CreateSessionCallbackProxy.CreateSession` (`GameplayStatics.GetPlayerController` 0) MaxPlayers bUseLAN
    (:`then`
      ;[1 0.6702 0.1962] In Case of Failure to load level (usually due to missing Steam Connection)
      (`KismetSystemLibrary.Delay` 20.0)
      (bind _returnvalue (`GameplayStatics.GetCurrentLevelName` true))
      (if (`KismetStringLibrary.EqualEqual_StrStr` _returnvalue "Map_MainMenu")
        (`KismetSystemLibrary.PrintString` "FailedToLoad. Try Again" true true (struct :`R` 0.154898 :`G` 1.0 :`A` 1.0) 5.0)
        (`self.Load_MainMenu`)))
    (:`OnSuccess`
      (`GameplayStatics.OpenLevel` (`KismetStringLibrary.Conv_StringToName` MapName) true "listen")
      (`self.SaveServerSettings` 360)
      (set `self.IsMultiplayer?` true)
      (`KismetSystemLibrary.Delay` 15.0)
      (bind _returnvalue_2 (`GameplayStatics.GetCurrentLevelName` true))
      (if (`KismetStringLibrary.EqualEqual_StrStr` _returnvalue_2 "Map_Transition")
        (`KismetSystemLibrary.PrintString` "FailedToLoad. Try Again" true true (struct :`R` 1.0 :`G` 0.033202 :`A` 1.0) 5.0)
        (`self.Load_MainMenu`)))
    (:`OnFailure`
      (`self.EndSession` null)
      (`KismetSystemLibrary.PrintString` "Failed to Load" true true (struct :`R` 1.0 :`G` 0.54016 :`A` 1.0) 8.0))))

(event `Join_Sessions`
  (params (Sesisons :type "BlueprintSessionResult Structure (by ref)"))
  ;[0.3005 0.3005 0.3005] Join Multiplayer Session (Client)
  (`JoinSessionCallbackProxy.JoinSession` (`GameplayStatics.GetPlayerController` 0) Sesisons))

(event `EndSession`
  (params (Client :type "PlayerController Object Reference"))
  ;[0.3005 0.3005 0.3005] End Session
  (`DestroySessionCallbackProxy.DestroySession` Client
    (:`OnSuccess`
      (`self.Load_MainMenu`))))

(event `Load_SP_Level`
  (params (LevelName :type Name))
  ;[0.3005 0.3005 0.3005] Load Singleplayer Session
  (`GameplayStatics.OpenLevel` LevelName)
  (set `self.IsMultiplayer?` false))

(event `Load_MainMenu`
  ;[0.3005 0.3005 0.3005] Load Main Menu
  (`GameplayStatics.OpenLevel` "Map_MainMenu" true "listen")
  (`self.SaveServerSettings` 1000))

(event `self.HandleNetworkError`
  (params (FailureType :type "ENetworkFailure Enum" :default "NetDriverAlreadyExists") (bIsServer :type Boolean))
  ;[0.3005 0.3005 0.3005] In Case of Error / Shutdown, go to Main Menu
  (`GameplayStatics.OpenLevel` "Map_MainMenu" true "listen" :!label _label))

(event `self.HandleTravelError`
  (params (FailureType :type "ETravelFailure Enum" :default "NoLevel"))
  ;[0.3005 0.3005 0.3005] In Case of Error / Shutdown, go to Main Menu
  (goto _label))

(event `self.ReceiveShutdown`
  ;[0.3005 0.3005 0.3005] In Case of Error / Shutdown, go to Main Menu
  (goto _label))

(event `SetVolume`
  (params (Volume :type Integer) (SoundClass :type "SoundClass Object Reference"))
  ;[0.3005 0.3005 0.3005] Set Master Volume
  (`GameplayStatics.SetSoundMixClassOverride` "/Game/MP_System_V3/Game/Sounds/SM_MPS.SM_MPS" SoundClass (/ (`KismetMathLibrary.Conv_IntToDouble` Volume) 100.0) 1.0 1.0 false))

(fn `LoadLoadout`
  (returns (Loadout :type "Array of /Game/MP_System_V3/Game/Blueprints/Core/BP_Weapon_Master Class Reference") (ID :type "Array of Integer") (SaveSlotID :type "Array of String"))
  (bind _returnvalue (`GameplayStatics.DoesSaveGameExist` (`self.SaveLoadoutSlot`)))
  (if _returnvalue
    (bind _returnvalue_2 (`GameplayStatics.LoadGameFromSlot` (`self.SaveLoadoutSlot`)))
    (bind _ass_save_loadout (cast `/Game/MP_System_V3/Game/Blueprints/SaveFiles/S_SaveLoadout` _returnvalue_2))
    (bind _output_get (set `self.SavedLoadout` _ass_save_loadout))
    (return (`/Game/MP_System_V3/Game/Blueprints/SaveFiles/S_SaveLoadout.Loadout` _output_get) (`/Game/MP_System_V3/Game/Blueprints/SaveFiles/S_SaveLoadout.ID` _output_get) (`/Game/MP_System_V3/Game/Blueprints/SaveFiles/S_SaveLoadout.SaveSlotID` _output_get))
    (else
      (bind _returnvalue_3 (`GameplayStatics.CreateSaveGameObject` "/Game/MP_System_V3/Game/Blueprints/SaveFiles/S_SaveLoadout.S_SaveLoadout_C"))
      (bind _output_get_2 (set `self.SavedLoadout` _returnvalue_3))
      (return (`/Game/MP_System_V3/Game/Blueprints/SaveFiles/S_SaveLoadout.Loadout` _output_get_2) (`/Game/MP_System_V3/Game/Blueprints/SaveFiles/S_SaveLoadout.ID` _output_get_2) (`/Game/MP_System_V3/Game/Blueprints/SaveFiles/S_SaveLoadout.SaveSlotID` _output_get_2)))))

(fn `LoadPlayerSettings`
  (returns (PlayerData :type "/Game/MP_System_V3/Game/Blueprints/Structs/ST_PlayerData Structure"))
  (bind _returnvalue (`GameplayStatics.DoesSaveGameExist` (`self.SavePlayerSettingsSlot`)))
  (if _returnvalue
    (bind _returnvalue_2 (`GameplayStatics.LoadGameFromSlot` (`self.SavePlayerSettingsSlot`)))
    (bind _ass_player_settings (cast `/Game/MP_System_V3/Game/Blueprints/SaveFiles/S_PlayerSettings` _returnvalue_2))
    (bind _output_get (set `self.SavedPlayerSettings` _ass_player_settings))
    (return (`/Game/MP_System_V3/Game/Blueprints/SaveFiles/S_PlayerSettings.PlayerData` _output_get))
    (else
      (bind _returnvalue_3 (`GameplayStatics.CreateSaveGameObject` "/Game/MP_System_V3/Game/Blueprints/SaveFiles/S_PlayerSettings.S_PlayerSettings_C"))
      (set `self.SavedPlayerSettings` _returnvalue_3))))

(fn `LoadServerSettings`
  (returns (MatchTime :type Integer))
  (bind _returnvalue (`GameplayStatics.LoadGameFromSlot` (`self.SaveSettingsSlot`)))
  (bind _ass_save_data (cast `/Game/MP_System_V3/Game/Blueprints/SaveFiles/S_SaveData` _returnvalue))
  (bind _output_get (set `self.SavedSettings` _ass_save_data))
  (return (`/Game/MP_System_V3/Game/Blueprints/SaveFiles/S_SaveData.MatchTime` _output_get)))

(fn `LoadSettings`
  (returns (PlayerNames :type "Array of Text") (Settings :type "/Game/MP_System_V3/Game/Blueprints/Structs/ST_SaveSettings Structure") (Stats :type "/Game/MP_System_V3/Game/Blueprints/Structs/ST_Stats Structure"))
  (bind _returnvalue (`GameplayStatics.DoesSaveGameExist` (`self.SaveSettingsSlot`)))
  (if _returnvalue
    (bind _returnvalue_2 (`GameplayStatics.LoadGameFromSlot` (`self.SaveSettingsSlot`)))
    (bind _ass_save_data (cast `/Game/MP_System_V3/Game/Blueprints/SaveFiles/S_SaveData` _returnvalue_2))
    (bind _output_get (set `self.SavedSettings` _ass_save_data))
    (return (`/Game/MP_System_V3/Game/Blueprints/SaveFiles/S_SaveData.PlayerNames` _output_get) (`/Game/MP_System_V3/Game/Blueprints/SaveFiles/S_SaveData.Settings` _output_get) (`/Game/MP_System_V3/Game/Blueprints/SaveFiles/S_SaveData.Stats` _output_get))
    (else
      (bind _returnvalue_3 (`GameplayStatics.CreateSaveGameObject` "/Game/MP_System_V3/Game/Blueprints/SaveFiles/S_SaveData.S_SaveData_C"))
      (set `self.SavedSettings` _returnvalue_3))))

(fn `SaveLoadout`
  (params (Loadout :type "Array of /Game/MP_System_V3/Game/Blueprints/Core/BP_Weapon_Master Class Reference") (ID :type "Array of Integer") (SaveSlotID :type "Array of String"))
  (bind _playercontroller (`/Game/MP_System_V3/Game/Blueprints/Core/FL_MPS.PlayerController_MPS`))
  (bind _savedloadout (`self.SavedLoadout`))
  (set `/Game/MP_System_V3/Game/Blueprints/SaveFiles/S_SaveLoadout.Loadout` Loadout _savedloadout)
  (set `/Game/MP_System_V3/Game/Blueprints/SaveFiles/S_SaveLoadout.ID` ID _savedloadout)
  (set `/Game/MP_System_V3/Game/Blueprints/SaveFiles/S_SaveLoadout.SaveSlotID` SaveSlotID _savedloadout)
  (`GameplayStatics.SaveGameToSlot` _savedloadout (`self.SaveLoadoutSlot`))
  (`/Engine/EditorBlueprintResources/StandardMacros.IsValid` _playercontroller
    (:`Is Valid`
      (`/Game/MP_System_V3/Game/Blueprints/Core/PC_MPS.RefreshLoadout` _playercontroller))))

(fn `SavePlayerSettings`
  (params (PlayerData :type "/Game/MP_System_V3/Game/Blueprints/Structs/ST_PlayerData Structure"))
  (bind _savedplayersettings (`self.SavedPlayerSettings`))
  (set `/Game/MP_System_V3/Game/Blueprints/SaveFiles/S_PlayerSettings.PlayerData` PlayerData _savedplayersettings)
  (`GameplayStatics.SaveGameToSlot` _savedplayersettings (`self.SavePlayerSettingsSlot`)))

(fn `SaveServerSettings`
  (params (MatchTime :type Integer))
  (bind _savedsettings (`self.SavedSettings`))
  (set `/Game/MP_System_V3/Game/Blueprints/SaveFiles/S_SaveData.MatchTime` MatchTime _savedsettings)
  (`GameplayStatics.SaveGameToSlot` _savedsettings (`self.SaveSettingsSlot`)))

(fn `SaveSettings`
  (params (PlayerNames :type "Array of Text") (Settings :type "/Game/MP_System_V3/Game/Blueprints/Structs/ST_SaveSettings Structure"))
  (bind _savedsettings (`self.SavedSettings`))
  (set `/Game/MP_System_V3/Game/Blueprints/SaveFiles/S_SaveData.Settings` Settings _savedsettings)
  (set `/Game/MP_System_V3/Game/Blueprints/SaveFiles/S_SaveData.PlayerNames` PlayerNames _savedsettings)
  (`GameplayStatics.SaveGameToSlot` _savedsettings (`self.SaveSettingsSlot`)))

(fn `SaveStats`
  (params (Stats :type "/Game/MP_System_V3/Game/Blueprints/Structs/ST_Stats Structure"))
  (bind _savedsettings (`self.SavedSettings`))
  (set `/Game/MP_System_V3/Game/Blueprints/SaveFiles/S_SaveData.Stats` Stats _savedsettings)
  (`GameplayStatics.SaveGameToSlot` _savedsettings (`self.SaveSettingsSlot`)))