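; BP_InteractionMaster is a base interactable item that shows its name in an interaction widget while unowned.
; Client_DrawWidget creates W_Interact once for the passed player, sets the item name and assigns it to the Info component.
; A retriggerable 0.4-second delay clears the widget and resets the gate once calls stop, avoiding explicit hide calls.
; Weapon and magazine interface functions are empty stubs.
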(event `Client_DrawWidget`
  (params (OwningPlayer :type "PlayerController Object Reference"))
  ;[0.3005 0.3005 0.3005] Overlap
  (if (not (`self.IsOwned?`))
    (`|ExecutionSequence`
      (:`then_0`
        (`/Engine/EditorBlueprintResources/StandardMacros.DoOnce` false :!label _label
          (:`Completed`
            (`|ExecutionSequence`
              (:`then_0`
                (`/Engine/EditorBlueprintResources/StandardMacros.DoOnce` false
                  (:`Completed`
                    (bind _returnvalue (`|CreateWidget` "/Game/MP_System_V3/Game/Blueprints/Widgets/W_Interact.W_Interact_C" OwningPlayer))
                    (bind _output_get (set `self.Widget_Info` _returnvalue))
                    (`TextBlock.SetText` (`/Game/MP_System_V3/Game/Blueprints/Widgets/W_Interact.Name` _output_get) (`self.ItemName`)))))
              (:`then_1`
                (`WidgetComponent.SetWidget` (`self.Info`) (`self.Widget_Info`)))))))
      (:`then_1`
        (`KismetSystemLibrary.RetriggerableDelay` 0.4)
        (`WidgetComponent.SetWidget` (`self.Info`) null)
        (goto _label :!via `Reset`)))))

(fn `I_Magazine`
  (returns (Magazine :type "/Game/MP_System_V3/Game/Blueprints/Core/BP_Magazine_Master Object Reference"))
  (return null))

(fn `I_Weapon`
  (returns (Weapon :type "/Game/MP_System_V3/Game/Blueprints/Core/BP_Weapon_Master Object Reference"))
  (return null))

(fn `UserConstructionScript`)