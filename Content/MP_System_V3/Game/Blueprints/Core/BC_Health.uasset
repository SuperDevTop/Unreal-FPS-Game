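; Health component that stores current health and regenerates it over time after a change.
; The Health function adds a signed amount to the current value and calls Healing, which starts a looping timer with an initial delay.
; Each Heal tick raises health within a clamped range, clearing the timer at full or otherwise sending a client update.
; The client update event fires an UpdateHealth dispatcher, but the final tick at full health skips it.
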(event `Healing`
  (bind _returnvalue (`KismetSystemLibrary.K2_SetTimer` null "Heal" 0.25 true 3.0))
  (set `self.HealTimer` _returnvalue))

(event `Client_Update`
  (params (Health :type "Float (double-precision)"))
  (`self.UpdateHealth` Health))

(fn `Heal`
  (bind _output_get (set `self.CurrentHealth` (`KismetMathLibrary.FClamp` (+ (`self.CurrentHealth`) 2.0) 0.0 100.0)))
  (if (>= _output_get 100.0)
    (`KismetSystemLibrary.K2_ClearAndInvalidateTimerHandle` (`self.HealTimer`))
    (else
      (`self.Client_Update` _output_get))))

(fn `Health`
  (params (InHealth :type "Float (double-precision)"))
  (returns (OutHealth :type "Float (double-precision)"))
  (bind _output_get (set `self.CurrentHealth` (+ InHealth (`self.CurrentHealth`))))
  (`self.Healing`)
  (return _output_get))