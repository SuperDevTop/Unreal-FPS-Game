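; Multiplayer game state that runs the session through WarmUp, PreMatch and Match phases and ends it when match time expires.
; On authority it loads match time from server settings, tracks players and runs a looping countdown that advances the replicated phase.
; The phase's OnRep multicasts dispatchers and starts each timer, with Match first polling for enough players.
; Session end disconnects active players, then closes the session through the game instance after a delay.
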(event `self.ReceiveBeginPlay`
  ;[0.3005 0.3005 0.3005] Event Begin Play
  (`/Engine/EditorBlueprintResources/ActorMacros.Switch Has Authority`
    (:`Authority`
      (bind _matchtime (`/Game/MP_System_V3/Game/Blueprints/Core/GI_MPS.LoadServerSettings` (`/Game/MP_System_V3/Game/Blueprints/Core/FL_MPS.GameInstance_MPS`)))
      (set `self.MatchTime` _matchtime)
      (set `self.GameStates` "NewEnumerator0")
      ;[0.3005 0.3005 0.3005] Update Players
      (add `/Game/MP_System_V3/Game/Blueprints/Core/GM_MPS.NewPlayer` (`/Game/MP_System_V3/Game/Blueprints/Core/FL_MPS.GameMode_MPS`) (delegate `AddNewPlayer`)))))

(event `AddNewPlayer`
  (bind _activeplayers (`self.ActivePlayers`))
  ;[0.3005 0.3005 0.3005] Update Players
  (for _array_element (`self.PlayerArray`)
    (if (not (`KismetArrayLibrary.Array_Contains` _activeplayers _array_element))
      (`KismetArrayLibrary.Array_Add` _activeplayers _array_element))))

(event `MC_GameStates`
  (params (Selection :type "/Game/MP_System_V3/Game/Blueprints/Enums/ENUM_GameStates Enum" :default "NewEnumerator0"))
  ;[0.3005 0.3005 0.3005] Replicate Dispatches to All
  (switch `/Game/MP_System_V3/Game/Blueprints/Enums/ENUM_GameStates` Selection
    (:`NewEnumerator0`
      (`self.Dispatch_WarmUp`))
    (:`NewEnumerator1`
      (`self.Dispatch_PreMatch`))
    (:`NewEnumerator2`
      (`self.Dispatch_Match`))))

(event `WaitForEnoughPlayers`
  ;[0.3005 0.3005 0.3005] Wait For Enough Players to Start the Game Time (Default 2 Players are needed)
  (`self.WaitForPlayers` 1
    (:`Start`
      (`self.StartTimer` (`self.MatchTime`))
      (set `self.GameActive` true))))

(event `Timer`
  ;[0.3005 0.3005 0.3005] Countdown Handle
  (bind _returnvalue (`KismetSystemLibrary.K2_SetTimerDelegate` (delegate `TimerRundown`) 1.0 true))
  (set `self.TimeHandle` _returnvalue))

(event `TimerRundown`
  ;[0.3005 0.3005 0.3005] Countdown Handle
  (bind _result (`/Engine/EditorBlueprintResources/StandardMacros.DecrementInt` (`self.Countdown_Time`))
    (:`  `
      (if (<= _result 0)
        (switch `/Game/MP_System_V3/Game/Blueprints/Enums/ENUM_GameStates` (`self.GameStates`)
          (:`NewEnumerator0`
            (set `self.GameStates` "NewEnumerator1"))
          (:`NewEnumerator1`
            (set `self.GameStates` "NewEnumerator2"))
          (:`NewEnumerator2`
            (`self.EndSession`)))))))

(fn `OnRep_GameStates`
  (bind _gamestates (`self.GameStates`))
  (`self.MC_GameStates` _gamestates)
  (switch `/Game/MP_System_V3/Game/Blueprints/Enums/ENUM_GameStates` _gamestates
    (:`NewEnumerator0`
      (`self.StartTimer` (`self.WarmUpTime`)))
    (:`NewEnumerator1`
      (`self.StartTimer` (`self.PreMatchTime`)))
    (:`NewEnumerator2`
      (`self.WaitForEnoughPlayers`))))

(fn `StartTimer`
  (params (Countdown_Time :type Integer))
  (`/Engine/EditorBlueprintResources/ActorMacros.Switch Has Authority`
    (:`Authority`
      (`self.StopTimer`)
      (set `self.Countdown_Time` Countdown_Time)
      (`self.Timer`))))

(fn `StopTimer`
  (`KismetSystemLibrary.K2_ClearAndInvalidateTimerHandle` (`self.TimeHandle`)))

(fn `UserConstructionScript`)