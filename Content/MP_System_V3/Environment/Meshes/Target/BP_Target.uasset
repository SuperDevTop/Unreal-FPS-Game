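; Shootable target actor that takes point and radial damage, falls under physics when destroyed, and updates record and scoreboard objective widgets.
; Point hits on hitable components remove one life each, while radial damage destroys it instantly.
; Type decides recovery: respawn types reset after a delay via server-to-multicast events; Trigger and Single Life use a separate respawn event pair.
; Swivel and AddItem are empty stubs here.
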(event `self.ReceiveRadialDamage`
  (params (DamageReceived :type "Float (single-precision)") (DamageType :type "DamageType Object Reference") (Origin :type "Vector Structure") (HitInfo :type "HitResult Structure (by ref)") (InstigatedBy :type "Controller Object Reference") (DamageCauser :type "Actor Object Reference"))
  ;[0.3005 0.3005 0.3005] Damage
  (if (`self.IsActive?`)
    (`PrimitiveComponent.SetSimulatePhysics` (`self.Target`) true :!label _label)
    (`self.TargetDestroyed`)
    (set `self.IsActive?` false)
    (`self.ReturnToState`)
    (`self.RecordHits`)
    (`|ExecutionSequence`
      (:`then_0`
        (switch `/Game/MP_System_V3/Environment/Meshes/Target/ENUM_Target` (`self.Type`)
          (:`NewEnumerator0`
            (`KismetSystemLibrary.Delay` (`self.Delay`) :!label _label_2)
            (`self.Svr_Respawn` (`StaticMeshComponent.StaticMesh` (`self.Target`))))
          (:`NewEnumerator1`
            (`KismetSystemLibrary.Delay` (`self.DestroyDelay`) :!label _label_3))
          (:`NewEnumerator3`
            (goto _label_2))
          (:`NewEnumerator2`
            (goto _label_3))))
      (:`then_1`
        (`KismetSystemLibrary.Delay` 0.1)
        (`GameplayStatics.PlaySound2D` "/Game/MP_System_V3/Game/Sounds/Cue/S_Hitmarker_Cue.S_Hitmarker_Cue" 2.0 1.0 0.0 null null)))))

(event `self.ReceivePointDamage`
  (params (Damage :type "Float (single-precision)") (DamageType :type "DamageType Object Reference") (HitLocation :type "Vector Structure") (HitNormal :type "Vector Structure") (HitComponent :type "PrimitiveComponent Object Reference") (BoneName :type Name) (ShotFromDirection :type "Vector Structure") (InstigatedBy :type "Controller Object Reference") (DamageCauser :type "Actor Object Reference") (HitInfo :type "HitResult Structure (by ref)"))
  ;[0.3005 0.3005 0.3005] Damage
  (if (`self.IsActive?`)
    (if (`KismetArrayLibrary.Array_Contains` (`self.HitableComponents`) HitComponent)
      (`self.Swivel` HitComponent)
      (set `self.HitCounter` (+ (`self.HitCounter`) 1))
      (bind _output_get (set `self.Life` (- (`self.Life`) (`KismetMathLibrary.Clamp` (`KismetMathLibrary.FTrunc` Damage) 1 1))))
      (if (<= _output_get 0)
        (goto _label)))))

(event `RecordHits`
  ;[0.3005 0.3005 0.3005] Record Hits to Widget
  (if (`self.RecordHits?`)
    (bind _foundwidgets (`WidgetBlueprintLibrary.GetAllWidgetsOfClass` "/Game/MP_System_V3/Game/Blueprints/Widgets/W_Record.W_Record_C"))
    (bind _output (`|GetArrayItem` _foundwidgets))
    (`/Engine/EditorBlueprintResources/StandardMacros.IsValid` _output
      (:`Is Valid`
        (`/Game/MP_System_V3/Game/Blueprints/Widgets/W_Record.UpdateTargets` _output))
      (:`Is Not Valid`
        _))
    (bind _foundwidgets_2 (`WidgetBlueprintLibrary.GetAllWidgetsOfClass` "/Game/MP_System_V3/Game/Blueprints/Widgets/W_Scoreboard.W_Scoreboard_C"))
    (bind _asw_objectives (cast `/Game/MP_System_V3/Game/Blueprints/Widgets/W_Objectives` (`PanelWidget.GetChildAt` (`/Game/MP_System_V3/Game/Blueprints/Widgets/W_Scoreboard.Objectives` (`|GetArrayItem` _foundwidgets_2)) 0) :!pure true))
    (bind _current_no (`/Game/MP_System_V3/Game/Blueprints/Widgets/W_Objectives.Current_No` _asw_objectives))
    (if (< _current_no (`/Game/MP_System_V3/Game/Blueprints/Widgets/W_Objectives.Goal_No` _asw_objectives))
      (bind _output_get (set `/Game/MP_System_V3/Game/Blueprints/Widgets/W_Objectives.Current_No` (+ _current_no 1) _asw_objectives))
      (`TextBlock.SetText` (`/Game/MP_System_V3/Game/Blueprints/Widgets/W_Objectives.Current` _asw_objectives) (`KismetTextLibrary.Conv_IntToText` _output_get)))))

(event `MC_Respawn`
  (params (NewMesh :type "StaticMesh Object Reference"))
  ;[0.3005 0.3005 0.3005] Respawn Target
  (switch `/Game/MP_System_V3/Environment/Meshes/Target/ENUM_Target` (`self.Type`)
    (:`NewEnumerator0`
      _)
    (:`NewEnumerator3`
      _))
  (`self.Reset`)
  (set `self.IsActive?` true)
  (set `self.Life` (`self.StoredLife`))
  (`self.RelocateAttachments`))

(event `Svr_Respawn`
  (params (NewMesh :type "StaticMesh Object Reference"))
  ;[0.3005 0.3005 0.3005] Respawn Target
  (`self.MC_Respawn` NewMesh))

(event `MC_SingleLifeRespawn`
  (params (Mesh :type "StaticMesh Object Reference"))
  ;[0.3005 0.3005 0.3005] Respawn on Trigger
  (switch `/Game/MP_System_V3/Environment/Meshes/Target/ENUM_Target` (`self.Type`)
    (:`NewEnumerator1`
      _)
    (:`NewEnumerator2`
      _))
  (`self.Reset`)
  (set `self.IsActive?` true)
  (set `self.Life` (`self.StoredLife`))
  (`self.RelocateAttachments`))

(event `Svr_SingleLifeRespawn`
  (params (Mesh :type "StaticMesh Object Reference"))
  ;[0.3005 0.3005 0.3005] Respawn on Trigger
  (`self.MC_SingleLifeRespawn` Mesh))

(event `Reset`
  (bind _target (`self.Target`))
  ;[0.3005 0.3005 0.3005] Reset Target Transforms
  (`PrimitiveComponent.SetSimulatePhysics` _target false)
  (`SceneComponent.K2_SetWorldTransform` _target (`self.TargetTransform`) false false))

(fn `AddItem`
  (returns (Item :type "PrimitiveComponent Object Reference"))
  (return null))

(fn `Swivel`
  (params (Component :type "PrimitiveComponent Object Reference"))
  (return))

(fn `UserConstructionScript`
  (`StaticMeshComponent.SetStaticMesh` (`self.Target`) (`self.TargetMesh`)))