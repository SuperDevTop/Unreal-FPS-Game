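; Moving shootable target variant that slides back and forth along its local X axis while it has Life.
; A looping timer, started through a Svr_ event, offsets the Target mesh and flips direction at fixed limits, clearing itself when Life runs out.
; InitiateMovement, bound to the return-to-state callback, recaptures the transform and restarts movement after a delay.
; The Target registers as a hitable component for the parent class.
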(event `self.ReceiveBeginPlay`
  (set `self.TargetTransform` (`SceneComponent.K2_GetComponentToWorld` (`self.Target`)))
  (set `self.StoredLife` (`self.Life`))
  (`self.Svr_Movement`)
  (add `self.ReturnToState` (delegate `InitiateMovement`)))

(event `InitiateMovement`
  (set `self.TargetTransform` (`SceneComponent.K2_GetComponentToWorld` (`self.Target`)))
  (`KismetSystemLibrary.Delay` (`self.Delay`))
  (`self.Svr_Movement`))

(event `Svr_Movement`
  (bind _returnvalue (`KismetSystemLibrary.K2_SetTimer` null "Movement" 0.01 true))
  (set `self.MovementTimer` _returnvalue))

(fn `AddItem`
  (returns (Item :type "PrimitiveComponent Object Reference"))
  (`parent.AddItem`)
  (return (`self.Target`)))

(fn `Movement`
  (if (> (`self.Life`) 0)
    (bind _target (`self.Target`)
      (:`then`
        (`SceneComponent.K2_AddLocalOffset` _target (`KismetMathLibrary.MakeVector` (`self.MoveSpeed`)) false false)
        (bind _output_get (set `self.TargetOffset` (+ (`self.TargetOffset`) (`self.MoveSpeed`))))
        (if (>= _output_get 100.0)
          (set `self.MoveSpeed` -1.0)
          (elif (<= _output_get -100.0)
            (set `self.MoveSpeed` 1.0))))
      (:`else`))
    (else
      (`KismetSystemLibrary.K2_ClearAndInvalidateTimerHandle` (`self.MovementTimer`)))))

(fn `UserConstructionScript`
  (`parent.UserConstructionScript`)
  (`KismetArrayLibrary.Array_Add` (`self.HitableComponents`) (`self.Target`)))