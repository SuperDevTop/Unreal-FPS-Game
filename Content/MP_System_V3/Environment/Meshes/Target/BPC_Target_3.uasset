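; Child target variant for a multiplayer target system, with a Base that rolls 90 degrees when its trigger is overlapped in the Trigger types.
; It registers the Target mesh as hittable and binds the parent's relocate and return-to-state hooks.
; Those hooks route through server-to-multicast events that re-attach the Target to the Base or roll the Base back.
; On return, timed triggers fire again, while others clear the overlap latch.
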(event `self.ReceiveBeginPlay`
  ;[0.3005 0.3005 0.3005] Rotations
  (set `self.TargetTransform` (`SceneComponent.K2_GetComponentToWorld` (`self.Target`)))
  (set `self.StoredLife` (`self.Life`))
  (add `self.RelocateAttachments` (delegate `Return`))
  (add `self.ReturnToState` (delegate `ReRotate`)))

(event `Return`
  ;[0.3005 0.3005 0.3005] Rotations
  (`self.Svr_Return`))

(event `ReRotate`
  ;[0.3005 0.3005 0.3005] Rotations
  (`self.Svr_ReRotate`))

(event `Svr_Return`
  ;[0.3005 0.3005 0.3005] Rotations
  (`self.MC_Return`))

(event `Svr_ReRotate`
  ;[0.3005 0.3005 0.3005] Rotations
  (`self.MC_ReRotate`))

(event `self.Trigger.OnComponentBeginOverlap`
  (params (OverlappedComponent :type "PrimitiveComponent Object Reference") (OtherActor :type "Actor Object Reference") (OtherComp :type "PrimitiveComponent Object Reference") (OtherBodyIndex :type Integer) (bFromSweep :type Boolean) (SweepResult :type "HitResult Structure (by ref)"))
  (bind _base (`self.Base`))
  (bind (_returnvalue_roll _returnvalue_pitch _returnvalue_yaw) (`KismetMathLibrary.BreakRotator` (`SceneComponent.K2_GetComponentRotation` _base)))
  ;[0.3005 0.3005 0.3005] Overlap Event
  (if (not (`self.Overlapped`)) :!label _label
    (set `self.Overlapped` true)
    (switch `/Game/MP_System_V3/Environment/Meshes/Target/ENUM_Target` (`self.Type`) :!label _label_2
      (:`NewEnumerator1`
        _)
      (:`NewEnumerator3`
        _))
    (`SceneComponent.K2_SetWorldRotation` _base (`KismetMathLibrary.MakeRotator` (- _returnvalue_roll 90.0) _returnvalue_pitch _returnvalue_yaw) false false)))

(event `Triggered`
  ;[0.3005 0.3005 0.3005] Overlap Event
  (goto _label))

(event `Retrigger`
  ;[0.3005 0.3005 0.3005] Overlap Event
  (goto _label_2))

(event `MC_Return`
  (bind _target (`self.Target`))
  ;[0.3005 0.3005 0.3005] Replicated Transforms
  (if (`self.TimedTrigger`)
    (`self.Retrigger`)
    (else
      (set `self.Overlapped` false)))
  (`SceneComponent.K2_AttachToComponent` _target (`self.Base`) "None" "SnapToTarget" "SnapToTarget" "KeepRelative" true)
  (`SceneComponent.K2_SetRelativeTransform` _target (`KismetMathLibrary.MakeTransform` (0.0 -6.0 0.0) (struct :`Yaw` 180.0)) false false))

(event `MC_ReRotate`
  (bind _base (`self.Base`))
  (bind (_returnvalue_roll _returnvalue_pitch _returnvalue_yaw) (`KismetMathLibrary.BreakRotator` (`SceneComponent.K2_GetComponentRotation` _base)))
  ;[0.3005 0.3005 0.3005] Replicated Transforms
  (`SceneComponent.K2_SetWorldRotation` _base (`KismetMathLibrary.MakeRotator` (+ _returnvalue_roll 90.0) _returnvalue_pitch _returnvalue_yaw) false false))

(fn `AddItem`
  (returns (Item :type "PrimitiveComponent Object Reference"))
  (`parent.AddItem`)
  (return (`self.Target`)))

(fn `UserConstructionScript`
  (`parent.UserConstructionScript`)
  (`KismetArrayLibrary.Array_Add` (`self.HitableComponents`) (`self.Target`)))