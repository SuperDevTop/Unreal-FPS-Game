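; BPC_Target_2 is a target Blueprint that extends a parent class, registering its Target component as hitable.
; The construction script runs the parent's setup, then adds Target to HitableComponents.
; BeginPlay caches Target's world transform and the starting Life value.
; The AddItem override calls the parent version and returns Target.
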(event `self.ReceiveBeginPlay`
  (set `self.TargetTransform` (`SceneComponent.K2_GetComponentToWorld` (`self.Target`)))
  (set `self.StoredLife` (`self.Life`)))

(fn `AddItem`
  (returns (Item :type "PrimitiveComponent Object Reference"))
  (`parent.AddItem`)
  (return (`self.Target`)))

(fn `UserConstructionScript`
  (`parent.UserConstructionScript`)
  (`KismetArrayLibrary.Array_Add` (`self.HitableComponents`) (`self.Target`)))