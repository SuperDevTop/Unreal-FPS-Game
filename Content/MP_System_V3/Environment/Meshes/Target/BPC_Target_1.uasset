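; BPC_Target_1 is a child target Blueprint with two hittable swivel pieces, apparently for multiplayer.
; On BeginPlay it stores the target's transform and life and hooks Swivels into relocate-attachment handling.
; Swivels passes through server and multicast events, which clear both meshes, restore them after a short delay and snap them to Target sockets.
; The Swivel override runs parent logic, then flips the given piece by half a turn.
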(event `self.ReceiveBeginPlay`
  (set `self.TargetTransform` (`SceneComponent.K2_GetComponentToWorld` (`self.Target`)))
  (set `self.StoredLife` (`self.Life`))
  (add `self.RelocateAttachments` (delegate `Swivels`)))

(event `Swivels`
  (`self.Svr_Swivel`))

(event `Svr_Swivel`
  (`self.MC_Swivel`))

(event `MC_Swivel`
  (`StaticMeshComponent.SetStaticMesh` (`self.Swivel_01`) null)
  (`StaticMeshComponent.SetStaticMesh` (`self.Swivel_02`) null)
  (`KismetSystemLibrary.Delay` 0.1)
  (`StaticMeshComponent.SetStaticMesh` (`self.Swivel_01`) "/Game/MP_System_V3/Environment/Meshes/Target/Swivel.Swivel")
  (`StaticMeshComponent.SetStaticMesh` (`self.Swivel_02`) "/Game/MP_System_V3/Environment/Meshes/Target/Swivel.Swivel")
  (`SceneComponent.K2_AttachToComponent` (`self.Swivel_01`) (`self.Target`) "Swivel_01" "SnapToTarget" "SnapToTarget" "KeepRelative" true)
  (`SceneComponent.K2_AttachToComponent` (`self.Swivel_02`) (`self.Target`) "Swivel_02" "SnapToTarget" "SnapToTarget" "KeepRelative" true))

(fn `AddItem`
  (returns (Item :type "PrimitiveComponent Object Reference"))
  (bind _item (`parent.AddItem`))
  (return _item))

(fn `Swivel`
  (params (Component :type "PrimitiveComponent Object Reference"))
  (`parent.Swivel` Component)
  (if (== Component (`self.Swivel_01`))
    (`SceneComponent.K2_AddLocalRotation` (`self.Swivel_01`) (struct :`Yaw` 180.0) false false)
    (else
      (`SceneComponent.K2_AddLocalRotation` (`self.Swivel_02`) (struct :`Yaw` 180.0) false false))))

(fn `UserConstructionScript`
  (bind _hitablecomponents (`self.HitableComponents`))
  (`parent.UserConstructionScript`)
  (`KismetArrayLibrary.Array_Add` _hitablecomponents (`self.Swivel_01`))
  (`KismetArrayLibrary.Array_Add` _hitablecomponents (`self.Swivel_02`)))