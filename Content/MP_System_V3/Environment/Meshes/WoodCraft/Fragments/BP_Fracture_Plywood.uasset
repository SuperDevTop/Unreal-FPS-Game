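; Breakable plywood prop that collapses once, when a BP_MPS_Master actor overlaps its trigger box.
; The intact mesh is swapped for pre-fractured cell meshes, hidden at construction, which then simulate physics.
; A collapse sound and particle system play, and the fragment loop spawns a dust emitter per piece at one shared offset.
; BeginPlay caches the fragment components and their world transforms, though these graphs never read the transforms.
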(event `self.ReceiveBeginPlay`
  ;[0.3005 0.3005 0.3005] Setup
  (bind _output_get (set `self.Components` (`|MakeArray` (`self.Wood_Broken_Cube_003_cell_017`) (`self.Wood_Broken_Cube_003_cell_013`) (`self.Wood_Broken_Cube_003_cell_019`) (`self.Wood_Broken_Cube_003_cell_020`) (`self.Wood_Broken_Cube_003_cell_021`) (`self.Wood_Broken_Cube_003_cell_008`) (`self.Wood_Broken_Cube_003_cell_023_cell`) (`self.Wood_Broken_Cube_003_cell_024`) (`self.Wood_Broken_Cube_003_cell_025`) (`self.Wood_Broken_Cube_003_cell_026`) (`self.Wood_Broken_Cube_003_cell_027_cell`) (`self.Wood_Broken_Cube_003_cell_027_cell_001`) (`self.Wood_Broken_Cube_003_cell_028_cell`) (`self.Wood_Broken_Cube_003_cell_028_cell_002`) (`self.Wood_Broken_Cube_003_cell_cell`) (`self.Wood_Broken_Cube_003_cell_cell_001`) (`self.Wood_Broken_Cube_003_cell_001_cell`) (`self.Wood_Broken_Cube_003_cell_001_cell_001`) (`self.Wood_Broken_Cube_003_cell_001_cell_002`) (`self.Wood_Broken_Cube_003_cell_002`) (`self.Wood_Broken_Cube_003_cell_004`) (`self.Wood_Broken_Cube_003_cell_005`) (`self.Wood_Broken_Cube_003_cell_010_cell`) (`self.Wood_Broken_Cube_003_cell_010_cell_001`) (`self.Wood_Broken_Cube_003_cell_010_cell_002`) (`self.Wood_Broken_Cube_003_cell_cell_cell`) (`self.Wood_Broken_Cube_003_cell_016`))))
  (for _array_element _output_get
    (`KismetArrayLibrary.Array_Add` (`self.Transforms`) (`SceneComponent.K2_GetComponentToWorld` _array_element))))

(event `self.Box.OnComponentBeginOverlap`
  (params (OverlappedComponent :type "PrimitiveComponent Object Reference") (OtherActor :type "Actor Object Reference") (OtherComp :type "PrimitiveComponent Object Reference") (OtherBodyIndex :type Integer) (bFromSweep :type Boolean) (SweepResult :type "HitResult Structure (by ref)"))
  (bind _staticmesh (`self.StaticMesh`))
  ;[0.3005 0.3005 0.3005] Destroy Event
  (cast `/Game/MP_System_V3/Game/Blueprints/Core/BP_MPS_Master` OtherActor)
  (`/Engine/EditorBlueprintResources/StandardMacros.DoOnce` false
    (:`Completed`
      (`GameplayStatics.PlaySoundAtLocation` "/Game/MP_System_V3/Game/Sounds/Cue/Collapse_Cue.Collapse_Cue" (`self.K2_GetActorLocation`) (struct) 5.0 1.0 0.0 null null null null)
      (`ActorComponent.SetActive` (`self.ParticleSystem`) true true)
      (`KismetSystemLibrary.Delay` 0.2)
      (`ActorComponent.SetActive` (`self.ParticleSystem`) true true)
      (`SceneComponent.SetHiddenInGame` _staticmesh true false)
      (`PrimitiveComponent.SetCollisionEnabled` _staticmesh "NoCollision")
      (`SceneComponent.SetHiddenInGame` (`self.Fragments`) false true)
      (for _array_element (`self.Components`)
        (`PrimitiveComponent.SetSimulatePhysics` _array_element true)
        (`GameplayStatics.SpawnEmitterAtLocation` "/Game/MP_System_V3/Game/Commons/Particles/P_Dust_Light.P_Dust_Light" (+ (`SceneComponent.K2_GetComponentLocation` (`self.ParticleSystem`)) (0.0 -100.0 0.0)) (struct) (40.0 4.0 4.0))))))

(fn `UserConstructionScript`
  (`SceneComponent.SetHiddenInGame` (`self.Fragments`) true true))