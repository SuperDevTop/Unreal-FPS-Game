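; BP_SurfaceDecal is a configurable decal actor for adding surface detail to the environment.
; Its construction script assigns M_SurfaceDecal to the Decal component and creates a dynamic material instance from it.
; It then pushes the actor's variables into that instance: color, albedo, surface, mask and normal textures, PBR surface scalars, and mask shaping controls such as grunge, contrast, gradient and sphere.
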(fn `UserConstructionScript`
  (bind _decal (`self.Decal`))
  ;[0.3005 0.3005 0.3005] Material Setup
  (`DecalComponent.SetDecalMaterial` _decal "/Game/MP_System_V3/Game/Commons/Materials/Masters/M_SurfaceDecal.M_SurfaceDecal")
  (bind _returnvalue (`DecalComponent.CreateDynamicMaterialInstance` _decal))
  (`MaterialInstanceDynamic.SetVectorParameterValue` _returnvalue "Color" (`self.Color`))
  ;[0.3005 0.3005 0.3005] Textures
  (`MaterialInstanceDynamic.SetTextureParameterValue` _returnvalue "Albedo" (`self.Albedo`))
  (`MaterialInstanceDynamic.SetTextureParameterValue` _returnvalue "Surface" (`self.Surface`))
  (`MaterialInstanceDynamic.SetTextureParameterValue` _returnvalue "Mask" (`self.Mask`))
  (`MaterialInstanceDynamic.SetTextureParameterValue` _returnvalue "Normal" (`self.Normal`))
  ;[0.3005 0.3005 0.3005] Basic Surface Properties
  (`MaterialInstanceDynamic.SetScalarParameterValue` _returnvalue "Normal Strength" (`self.NormalStrength`))
  (`MaterialInstanceDynamic.SetScalarParameterValue` _returnvalue "Roughness" (`self.Roughness`))
  (`MaterialInstanceDynamic.SetScalarParameterValue` _returnvalue "Specular" (`self.Specular`))
  (`MaterialInstanceDynamic.SetScalarParameterValue` _returnvalue "Metalness" (`self.Metalness`))
  ;[0.3005 0.3005 0.3005] Mask
  (`MaterialInstanceDynamic.SetScalarParameterValue` _returnvalue "GrungeTakeover" (`self.GrungeTakeover`))
  (`MaterialInstanceDynamic.SetScalarParameterValue` _returnvalue "Opacity" (`self.Opacity`))
  (`MaterialInstanceDynamic.SetScalarParameterValue` _returnvalue "Contrast" (`self.Contrast`))
  (`MaterialInstanceDynamic.SetScalarParameterValue` _returnvalue "MaskContrast" (`self.MaskContrast`))
  (`MaterialInstanceDynamic.SetScalarParameterValue` _returnvalue "BottomGradient" (`self.BottomGradient`))
  (`MaterialInstanceDynamic.SetScalarParameterValue` _returnvalue "Sphere" (`self.Sphere`)))