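; BP_Decal is a configurable decal actor for dressing environments.
; Its construction script assigns M_DecalMaster to the Decal component and creates a dynamic material instance from it.
; The actor's variables drive that instance's color, alpha texture, scale, size and opacity parameters, so a single master material serves differently styled decals.
; It runs no gameplay logic, as BeginPlay and Tick are disabled.
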(fn `UserConstructionScript`
  (bind _decal (`self.Decal`))
  (`DecalComponent.SetDecalMaterial` _decal "/Game/MP_System_V3/Game/Commons/Materials/Masters/M_DecalMaster.M_DecalMaster")
  (bind _returnvalue (`DecalComponent.CreateDynamicMaterialInstance` _decal))
  (`MaterialInstanceDynamic.SetVectorParameterValue` _returnvalue "Color" (`self.Color`))
  (`MaterialInstanceDynamic.SetTextureParameterValue` _returnvalue "Alpha" (`self.Alpha`))
  (`MaterialInstanceDynamic.SetScalarParameterValue` _returnvalue "X" (`self.Scale_X`))
  (`MaterialInstanceDynamic.SetScalarParameterValue` _returnvalue "Y" (`self.Scale_Y`))
  (`MaterialInstanceDynamic.SetScalarParameterValue` _returnvalue "Size_X" (`self.Size_X`))
  (`MaterialInstanceDynamic.SetScalarParameterValue` _returnvalue "Size_Y" (`self.Size_Y`))
  (`MaterialInstanceDynamic.SetScalarParameterValue` _returnvalue "Opacity" (`self.Opacity`)))