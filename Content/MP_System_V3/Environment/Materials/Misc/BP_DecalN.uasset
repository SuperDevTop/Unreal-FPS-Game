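; BP_DecalN is a configurable decal actor for placing tinted, normal-mapped decals in the environment.
; Its construction script assigns M_RandomDecal to the Decal component and creates a dynamic material instance from it.
; The actor's variables drive that instance's color, alpha and normal textures, tiling or scale, angle, normal strength and roughness, so each placed decal can be customized individually.
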(fn `UserConstructionScript`
  (bind _decal (`self.Decal`))
  (`DecalComponent.SetDecalMaterial` _decal "/Game/MP_System_V3/Game/Commons/Materials/Masters/M_RandomDecal.M_RandomDecal")
  (bind _returnvalue (`DecalComponent.CreateDynamicMaterialInstance` _decal))
  (`MaterialInstanceDynamic.SetVectorParameterValue` _returnvalue "Color" (`self.Color`))
  (`MaterialInstanceDynamic.SetTextureParameterValue` _returnvalue "Alpha" (`self.Alpha`))
  (`MaterialInstanceDynamic.SetTextureParameterValue` _returnvalue "Normal" (`self.Normal`))
  (`MaterialInstanceDynamic.SetScalarParameterValue` _returnvalue "X" (`self.Scale_X`))
  (`MaterialInstanceDynamic.SetScalarParameterValue` _returnvalue "Y" (`self.Scale_Y`))
  (`MaterialInstanceDynamic.SetScalarParameterValue` _returnvalue "Scale" (`self.Scale`))
  (`MaterialInstanceDynamic.SetScalarParameterValue` _returnvalue "Normal Strength" (`self.NormalStrength`))
  (`MaterialInstanceDynamic.SetScalarParameterValue` _returnvalue "Roughness" (`self.Roughness`))
  (`MaterialInstanceDynamic.SetScalarParameterValue` _returnvalue "Angle" (`self.Angle`)))